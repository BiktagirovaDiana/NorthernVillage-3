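; BP_Tree is a choppable tree that the player and named residents can target.
; A trigger box sets the player's CanChop flag, caching the player so AnimChopTree can tilt the mesh by player-relative direction through a timeline, then reverse it.
; Residents reserve and release the tree by row name, query availability and get a chop location.
; The Chop event is an empty stub, and IsChopped is only read here.
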(event OnComponentBeginOverlap(Box)
  (params (OverlappedComponent :type Primitive%20Component%20Object%20Reference) (OtherActor :type Actor%20Object%20Reference) (OtherComp :type Primitive%20Component%20Object%20Reference) (OtherBodyIndex :type Integer) (bFromSweep :type Boolean) (SweepResult :type Hit%20Result%20Structure%20%28by%20ref%29))
  (bind _asbp_player_character (Utilities|Casting|CastToBP_PlayerCharacter OtherActor))
  (bind _output_get (Variables|Default|SetAs%20BP%20Player%20Character _asbp_player_character))
  (Variables|/Game/BluePrints/Player/BP_PlayerCharacter.BP_PlayerCharacter_C|SetCanChop _output_get true))

(event OnComponentEndOverlap(Box)
  (params (OverlappedComponent :type Primitive%20Component%20Object%20Reference) (OtherActor :type Actor%20Object%20Reference) (OtherComp :type Primitive%20Component%20Object%20Reference) (OtherBodyIndex :type Integer))
  (bind _asbp_player_character (Utilities|Casting|CastToBP_PlayerCharacter OtherActor))
  (Variables|/Game/BluePrints/Player/BP_PlayerCharacter.BP_PlayerCharacter_C|SetCanChop _asbp_player_character false))

(event Custom|Chop)

(event Custom|AnimChopTree
  (Variables|Default|SetA "0, 0, 0")
  (CallFunction|CheckDirection)
  (bind _alpha (Timeline|ChopTree Play)
    (:Update
      (Transformation|SetRelativeRotation (Variables|Default|GetStaticMesh) (Math|Rotator|Lerp(Rotator) (Variables|Default|GetA) (Variables|Default|GetB) _alpha) false false))
    (:Finished
      (CallFunction|CheckDirection)
      (Timeline|ChopTree Reverse))))

(event Custom|CheckDirection
  (bind _returnvalue (Transformation|GetActorTransform))
  (bind _as_bp_player_character (Variables|Default|GetAs%20BP%20Player%20Character))
  (bind _defaultsceneroot (Variables|Default|GetDefaultSceneRoot))
  (bind _returnvalue_2 (Transformation|GetWorldLocation _defaultsceneroot))
  (bind _rootcomponent (Variables|/Script/Engine.Actor|GetRootComponent _as_bp_player_character))
  (bind _returnvalue_3 (Transformation|GetWorldLocation _rootcomponent))
  (bind _returnvalue_4 (- _returnvalue_3 _returnvalue_2))
  (bind _returnvalue_5 (Math|Transform|InverseTransformDirection _returnvalue _returnvalue_4))
  (bind _returnvalue_6 (Math|Vector|Normalize _returnvalue_5))
  (bind _returnvalue_7 (!= (.y _returnvalue_6) 0.0))
  (bind _returnvalue_8 (* (.y _returnvalue_6) 5.0))
  (if (!= (.x _returnvalue_6) 0.0)
    (if _returnvalue_7
      (Variables|Default|SetB (Math|Rotator|MakeRotator 0.0 _returnvalue_8 0.0)))
    (Variables|Default|SetB (Math|Rotator|MakeRotator (* (.x _returnvalue_6) 5.0) 0.0 0.0))
    (elif _returnvalue_7
      (Variables|Default|SetB (Math|Rotator|MakeRotator 0.0 _returnvalue_8 0.0)))))

(event EventBeginPlay)

(event Collision|EventActorBeginOverlap
  (params (OtherActor :type Actor%20Object%20Reference)))

(event EventTick
  (params (DeltaSeconds :type Float%20%28single-precision%29)))

(fn ConstructionScript)

(fn IsFree
  (return (and (not (Variables|Default|GetbReserved)) (not (Variables|Default|GetIsChopped)))))

(fn Reserve
  (params (ResidentRowName :type Name))
  (if (not (Variables|Default|GetbReserved))
    (Variables|Default|SetbReserved true)
    (Variables|Default|SetReservedBy ResidentRowName)
    (return true)
    (else
      (return false))))

(fn GetChopLocation
  (return (Transformation|GetWorldLocation (Variables|Default|GetChopPoint))))

(fn Release
  (params (Resident%20Row%20Name :type Name))
  (if (and (== (Variables|Default|GetbReserved) true) (== (Variables|Default|GetReservedBy) Resident%20Row%20Name))
    (Variables|Default|SetbReserved false)
    (Variables|Default|SetReservedBy "None")
    (return true)
    (else
      (return false))))

(fn CanbeChoppedNow
  (return (not (Variables|Default|GetIsChopped))))