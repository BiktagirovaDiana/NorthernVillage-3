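; BP_Fire is a buildable fire that warms the player, burns wood as fuel and cooks items.
; Looping timers advance the burn clock and fuel bar while built, consume overlapping wood to rewind that clock, and scan for cookable items.
; Cooking swaps an item's data from DT_ItemsInventor after a delay and starts steam.
; WarmCollision overlaps set the player's IsCold flag based on built and burning state.
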(event OnComponentBeginOverlap(WarmCollision)
  (params (OverlappedComponent :type Primitive%20Component%20Object%20Reference) (OtherActor :type Actor%20Object%20Reference) (OtherComp :type Primitive%20Component%20Object%20Reference) (OtherBodyIndex :type Integer) (bFromSweep :type Boolean) (SweepResult :type Hit%20Result%20Structure%20%28by%20ref%29))
  (bind _asbp_player_character (Utilities|Casting|CastToBP_PlayerCharacter OtherActor))
  (if (Variables|Default|GetisBuilt)
    (if (Variables|Default|GetisBurn)
      (Variables|/Game/BluePrints/Player/BP_SlidersComponent.BP_SlidersComponent_C|SetisCold (Variables|/Game/BluePrints/Player/BP_PlayerCharacter.BP_PlayerCharacter_C|GetBP_SlidersComponent _asbp_player_character) false)
      (else
        (Variables|/Game/BluePrints/Player/BP_SlidersComponent.BP_SlidersComponent_C|SetisCold (Variables|/Game/BluePrints/Player/BP_PlayerCharacter.BP_PlayerCharacter_C|GetBP_SlidersComponent _asbp_player_character) true)))
    (else
      (Variables|/Game/BluePrints/Player/BP_SlidersComponent.BP_SlidersComponent_C|SetisCold (Variables|/Game/BluePrints/Player/BP_PlayerCharacter.BP_PlayerCharacter_C|GetBP_SlidersComponent _asbp_player_character) true))))

(event OnComponentEndOverlap(WarmCollision)
  (params (OverlappedComponent :type Primitive%20Component%20Object%20Reference) (OtherActor :type Actor%20Object%20Reference) (OtherComp :type Primitive%20Component%20Object%20Reference) (OtherBodyIndex :type Integer))
  (Utilities|Casting|CastToBP_Item OtherActor
    (:then
      (Variables|Default|SetisCook false)
      (Utilities|IsValid (Variables|Default|GetHoldItem)
        (:Is%20Valid
          (Variables|/Game/BluePrints/BP_Item.BP_Item_C|SetisBurn (Variables|Default|GetHoldItem) true)
          (Variables|Default|SetHoldItem 0))))
    (:CastFailed
      (bind _asbp_player_character (Utilities|Casting|CastToBP_PlayerCharacter OtherActor))
      (Variables|/Game/BluePrints/Player/BP_SlidersComponent.BP_SlidersComponent_C|SetisCold (Variables|/Game/BluePrints/Player/BP_PlayerCharacter.BP_PlayerCharacter_C|GetBP_SlidersComponent _asbp_player_character) true))))

(event Custom|Burn
  (if (Variables|Default|GetisBuilt)
    (Default|UpdateBar (Variables|Default|GetWBP%20Fire%20Bar) (Variables|Default|GetTimer) (Variables|Default|GetTime))
    (if (<= (Variables|Default|GetTime) (Variables|Default|GetTimer))
      (Variables|Default|SetisBurn true)
      (Variables|Default|SetTime (+ (Variables|Default|GetTime) 1.0))
      (else
        (Variables|Default|SetisBurn false)))))

(event Custom|Cook
  (params (RowName :type Name) (Timer :type Float%20%28double-precision%29) (Target :type BP%20Item%20Object%20Reference))
  (bind _returnvalue (Utilities|Time|SetTimerbyEvent (delegate Custom|Cooking) 0.5 true))
  (Variables|Default|SetTimerCook _returnvalue))

(event Custom|Cooking
  (if (Variables|Default|GetisCook)
    (bind _output_get (Variables|Default|SetTime (+ 0.5 (Variables|Default|GetTime))))
    (if (>= _output_get (stale Custom|Cook Timer))
      (bind _returnvalue (Utilities|GetDataTableRow "/Game/BluePrints/Resources/DT_ItemsInventor.DT_ItemsInventor" (stale Custom|Cook RowName))
        (:then
          (Default|ApplyItemData (stale Custom|Cook Target) (Utilities|Struct|MakeSTR_ItemsInventory (.name _returnvalue) (.icon _returnvalue) (.mesh _returnvalue) (.stackabled _returnvalue) (.quanity _returnvalue) (.maxstackebled _returnvalue) (.scale _returnvalue) (.enum _returnvalue) (.location _returnvalue) (.rotation _returnvalue)))
          (Default|StartSteam (stale Custom|Cook Target))
          (Utilities|Time|ClearandInvalidateTimerbyHandle (Variables|Default|GetTimerCook)))))
    (else
      (Utilities|Time|ClearandInvalidateTimerbyHandle (Variables|Default|GetTimerCook)))))

(event Custom|CheckWood
  (if (>= (Variables|Default|GetTime) 2e+01)
    (bind _array_element (Utilities|Array|ForEachLoopwithBreak (Collision|GetOverlappingActors (Variables|Default|GetWarm%20Collision) "/Game/BluePrints/BP_Item.BP_Item_C" :!class /Script/Engine.PrimitiveComponent) :!label _label)
      (:LoopBody
        (bind _asbp_item (Utilities|Casting|CastToBP_Item _array_element))
        (switch Utilities|FlowControl|Switch|SwitchonENUM_Item (.Enum (Utilities|Struct|BreakSTR_ItemsInventory (Variables|/Game/BluePrints/BP_Item.BP_Item_C|GetItem _asbp_item)))
          (:NewEnumerator10
            (Actor|DestroyActor _asbp_item)
            (Variables|Default|SetTime (- (Variables|Default|GetTime) 2e+01))
            (Default|UpdateBar (Variables|Default|GetWBP%20Fire%20Bar) (Variables|Default|GetTimer) (Variables|Default|GetTime))
            (goto _label Break)))))))

(event Custom|CheckCook
  (for _array_element (Collision|GetOverlappingActors (Variables|Default|GetWarm%20Collision) "/Game/BluePrints/BP_Item.BP_Item_C" :!class /Script/Engine.PrimitiveComponent)
    (bind _asbp_item (Utilities|Casting|CastToBP_Item _array_element))
    (switch Utilities|FlowControl|Switch|SwitchonENUM_Item (.Enum (Utilities|Struct|BreakSTR_ItemsInventory (Variables|/Game/BluePrints/BP_Item.BP_Item_C|GetItem _asbp_item)))
      (:NewEnumerator7
        (Variables|Default|SetisCook true)
        (CallFunction|Cook "Bucket_ColdWater3" 1e+01 _asbp_item))
      (:NewEnumerator18
        (Variables|Default|SetisCook true)
        (CallFunction|Cook "Bucket_Water3" 5.0 _asbp_item))
      (:NewEnumerator8
        (Variables|Default|SetisCook true)
        (CallFunction|Cook "Fried_Fish" 5.0 _asbp_item))
      (:NewEnumerator10
        (Variables|/Game/BluePrints/BP_Item.BP_Item_C|SetisBurn _asbp_item true)))))

(event Custom|CheckPlayer
  (if (Variables|Default|GetisBuilt)
    (if (Variables|Default|GetisBurn)
      (Utilities|Array|ForEachLoopwithBreak (Collision|GetOverlappingActors (Variables|Default|GetWarm%20Collision) "/Game/BluePrints/Player/BP_PlayerCharacter.BP_PlayerCharacter_C" :!class /Script/Engine.PrimitiveComponent)
        (:Completed
          (Variables|/Game/BluePrints/Player/BP_SlidersComponent.BP_SlidersComponent_C|SetisCold (Variables|/Game/BluePrints/Player/BP_PlayerCharacter.BP_PlayerCharacter_C|GetBP_SlidersComponent (Variables|Default|GetPlayer%20Character)) false))))))

(event EventBeginPlay
  (Variables|Default|SetisBurn true)
  (bind _asbp_player_character (Utilities|Casting|CastToBP_PlayerCharacter (Game|Player|GetPlayerPawn 0)))
  (Variables|Default|SetPlayer%20Character _asbp_player_character)
  (Variables|/Game/BluePrints/Player/BP_SlidersComponent.BP_SlidersComponent_C|SetisCold (Variables|/Game/BluePrints/Player/BP_PlayerCharacter.BP_PlayerCharacter_C|GetBP_SlidersComponent _asbp_player_character) false)
  (Rendering|SetVisibility (Variables|Default|GetWidget) true false)
  (bind _aswbp_fire_bar (Utilities|Casting|CastToWBP_FireBar (UserInterface|GetUserWidgetObject (Variables|Default|GetWidget))))
  (Variables|Default|SetWBP%20Fire%20Bar _aswbp_fire_bar)
  (Variables|Default|SetTimer 1e+02)
  (Variables|Default|SetTime 5e+01)
  (Utilities|Time|SetTimerbyEvent (delegate Custom|Burn) 1.0 true)
  (bind _returnvalue (Utilities|Time|SetTimerbyEvent (delegate Custom|CheckWood) 3.0 true))
  (Variables|Default|SetTimerWood _returnvalue)
  (Utilities|Time|SetTimerbyEvent (delegate Custom|CheckCook) 5.5 true))

(event Collision|EventActorBeginOverlap
  (params (OtherActor :type Actor%20Object%20Reference))
  (bind _asbp_player_character (Utilities|Casting|CastToBP_PlayerCharacter OtherActor))
  (Variables|/Game/BluePrints/Player/BP_SlidersComponent.BP_SlidersComponent_C|SetisCold (Variables|/Game/BluePrints/Player/BP_PlayerCharacter.BP_PlayerCharacter_C|GetBP_SlidersComponent _asbp_player_character) false))

(event EventTick
  (params (DeltaSeconds :type Float%20%28single-precision%29)))

(fn ConstructionScript
  (|CallParentFunction))