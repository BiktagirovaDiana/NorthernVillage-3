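; Base villager NPC that works as a fisherman or woodcutter, gets hungry and dies at zero hunger, destroying its home tent.
; Job changes from BP_IceHoleManager start looping timers that reserve the assigned ice hole or nearest free tree.
; AIMoveTo and a work timer drive each routine, adding fish or wood to inventory before walking home.
; A looping drain updates the hunger widget, while box overlap, FeedNPC and TakeLoot support player interaction.
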(event OnComponentBeginOverlap(Box)
  (params (OverlappedComponent :type Primitive%20Component%20Object%20Reference) (OtherActor :type Actor%20Object%20Reference) (OtherComp :type Primitive%20Component%20Object%20Reference) (OtherBodyIndex :type Integer) (bFromSweep :type Boolean) (SweepResult :type Hit%20Result%20Structure%20%28by%20ref%29))
  (bind _asbp_player_character (Utilities|Casting|CastToBP_PlayerCharacter OtherActor))
  (Default|SetCurrentInteractable (Actor|GetComponentbyClass _asbp_player_character "/Game/BluePrints/Player/BP_InteractionComponent.BP_InteractionComponent_C") self))

(event OnComponentEndOverlap(Box)
  (params (OverlappedComponent :type Primitive%20Component%20Object%20Reference) (OtherActor :type Actor%20Object%20Reference) (OtherComp :type Primitive%20Component%20Object%20Reference) (OtherBodyIndex :type Integer))
  (bind _asbp_player_character (Utilities|Casting|CastToBP_PlayerCharacter OtherActor))
  (Default|ClearCurrentInteractable (Actor|GetComponentbyClass _asbp_player_character "/Game/BluePrints/Player/BP_InteractionComponent.BP_InteractionComponent_C") self))

(event Custom|TryStartFishingRoutine
  (if (not (Variables|Default|GetbRoutineRunning))
    (Utilities|IsValid (Variables|Default|GetIceHoleManagerRef)
      (:Is%20Valid
        (bind _job (Default|GetResidentJob (Variables|Default|GetIceHoleManagerRef) (Variables|Default|GetResidentRowName)))
        (if (Utilities|Enum|Equal(Enum) _job "Рыбак")
          (bind _hole (Default|GetResidentHole (Variables|Default|GetIceHoleManagerRef) (Variables|Default|GetResidentRowName)))
          (Utilities|IsValid _hole
            (:Is%20Valid
              (Development|PrintString "валиден hole")
              (Variables|Default|SetAssignedHole _hole)
              (bind _success (Default|Reserve (Variables|Default|GetAssignedHole) (Variables|Default|GetResidentRowName)))
              (if _success
                (Variables|Default|SetbRoutineRunning true)
                (Development|PrintString "перед перым ai move")
                (Rendering|Debug|DrawDebugSphere (Default|GetFishingLocation (Variables|Default|GetAssignedHole)) 3e+01 12 "(R=1.000000,G=0.000000,B=0.035228,A=1.000000)" 1e+01)
                (AI|AIMoveTo self (Default|GetFishingLocation (Variables|Default|GetAssignedHole)) 0 3e+01 true
                  (:OnSuccess
                    (Development|PrintString "после1 ai move - удача")
                    (CallFunction|OnArrivedtoHole))
                  (:OnFail
                    (Development|PrintString "после1 ai move - проигрыш")
                    (CallFunction|AbortRoutine)))))))))))

(event Custom|OnArrivedToHole
  (Utilities|IsValid (Variables|Default|GetAssignedHole)
    (:Is%20Valid
      (Development|PrintString "пошли дальше")
      (Transformation|SetActorRotation (Math|Rotator|FindLookatRotation (Transformation|GetActorLocation) (Transformation|GetActorLocation (Variables|Default|GetAssignedHole))))
      (Development|PrintString "перед таймером")
      (Variables|Default|SetFishCount (Math|Random|RandomIntegerinRange 1 5))
      (bind _returnvalue (Utilities|Time|SetTimerbyEvent (delegate Custom|OnFishingFinished) 5.0))
      (Variables|Default|SetFishingTimerHandle _returnvalue))
    (:Is%20Not%20Valid
      (CallFunction|AbortRoutine))))

(event Custom|AbortWoodcutRoutine
  (Development|PrintString "все плохо")
  (Utilities|Time|ClearandInvalidateTimerbyHandle (Variables|Default|GetWoodcutTimerHandle))
  (AI|Navigation|StopMovement (Pawn|GetController))
  (Utilities|IsValid (Variables|Default|GetAssignedTree)
    (:Is%20Valid
      (Default|Release (Variables|Default|GetAssignedTree) (Variables|Default|GetResidentRowName))
      (Variables|Default|SetAssignedTree 0)
      (Variables|Default|SetbRoutineRunning false))))

(event Custom|job
  (params (ResidentRowName :type Name) (NewJob :type String))
  (if (== ResidentRowName (Variables|Default|GetResidentRowName))
    (switch string NewJob
      (:Рыбак
        (Utilities|Time|SetTimerbyEvent (delegate Custom|TryStartFishingRoutine) 2.0 true))
      (:Лесоруб
        (Utilities|Time|SetTimerbyEvent (delegate Custom|TryStartWoodcutRoutine) 2.0 true)))))

(event Custom|TryStartWork
  (bind _iceholemanagerref (Variables|Default|GetIceHoleManagerRef))
  (bind _residentrowname (Variables|Default|GetResidentRowName))
  (if (Variables|Default|GetbRoutineRunning)
    (Utilities|IsValid _iceholemanagerref
      (:Is%20Valid
        (bind _job (Default|GetResidentJob _iceholemanagerref _residentrowname))
        (switch string _job
          (:Рыбак
            (bind (_hole _success) (Default|AssignHoletoResident _iceholemanagerref _residentrowname))
            (if _success
              (Variables|Default|SetAssignedHole _hole)
              (Variables|Default|SetbRoutineRunning true)
              (CallFunction|TryStartFishingRoutine)
              (else
                (Utilities|Time|SetTimerbyEvent (delegate Custom|TryStartWork) 5.0)))))))))

(event Custom|InitFromData
  (bind _residentdata (Variables|Default|GetResidentData))
  (bind _mesh (Variables|Character|GetMesh))
  (bind (_displayname _portrait _npcclass _skeletalmesh _animbp) (Utilities|Struct|BreakSTR_ResidentCard _residentdata))
  (Components|SkeletalMesh|SetSkeletalMeshAsset _mesh _skeletalmesh)
  (Components|SkeletalMesh|SetAnimInstanceClass _mesh _animbp))

(event Custom|DrainHunger
  (bind _output_get (Variables|Default|SetHunger (Math|Float|Clamp(Float) (- (Variables|Default|GetHunger) (/ (Variables|Default|GetHungerTickInterval) 1.2e+02)))))
  (if (<= _output_get 0.0)
    (CallFunction|Die)
    (else
      (Default|UpdateHungerBar (Variables|Default|GetHungerWidgetRef)))))

(event Custom|Die
  (bind _hometent (Variables|Default|GetHomeTent))
  (if (Variables|Default|GetIsDead)
    (Development|PrintString "умерло")
    (else
      (Variables|Default|SetIsDead true)
      (Utilities|Time|ClearandInvalidateTimerbyHandle (Variables|Default|GetHungerTimerHandle))
      (Utilities|IsValid (Variables|Default|GetHungerWidgetRef)
        (:Is%20Valid
          (Rendering|SetVisibility (Variables|Default|GetWC_HungerBar) false false)
          (Utilities|IsValid _hometent
            (:Is%20Valid
              (Actor|DestroyActor _hometent)
              (Development|PrintString "убить лом"))
            (:Is%20Not%20Valid
              _))
          (Actor|DestroyActor self)
          (Development|PrintString "убить ии"))
        (:Is%20Not%20Valid
          (Development|PrintString "голод не валиден"))))))

(event Custom|AbortRoutine
  (Development|PrintString "все плохо")
  (Utilities|Time|ClearandInvalidateTimerbyHandle (Variables|Default|GetFishingTimerHandle))
  (AI|Navigation|StopMovement (Pawn|GetController))
  (Utilities|IsValid (Variables|Default|GetAssignedHole)
    (:Is%20Valid
      (Default|Release (Variables|Default|GetAssignedHole) (Variables|Default|GetResidentRowName))
      (Variables|Default|SetAssignedHole 0)
      (Variables|Default|SetbRoutineRunning false))))

(event Custom|OnFishingFinished
  (bind _residentrowname (Variables|Default|GetResidentRowName))
  (bind _hometent (Variables|Default|GetHomeTent))
  (Development|PrintString "действие ухода")
  (Utilities|IsValid (Variables|Default|GetAssignedHole)
    (:Is%20Valid
      (if (> (Variables|Default|GetFishCount) 0)
        (Default|AddItem (Variables|Default|GetInventoryComp) (Utilities|Struct|MakeSTR_ItemsInventory "Fish_Raw" 0 0 false (Variables|Default|GetFishCount)))
        (Default|Release (Variables|Default|GetAssignedHole) _residentrowname)
        (Variables|/Game/BluePrints/Resources/BP_WaterSource_IceHole.BP_WaterSource_IceHole_C|SetbIsOccupied (Variables|Default|GetAssignedHole) false)
        (Variables|/Game/BluePrints/Resources/BP_WaterSource_IceHole.BP_WaterSource_IceHole_C|SetOccupiedByResident (Variables|Default|GetAssignedHole) "None")
        (Default|ClearResidentHole (Variables|Default|GetIceHoleManagerRef) _residentrowname)
        (Variables|Default|SetAssignedHole 0)
        (Utilities|IsValid _hometent
          (:Is%20Valid
            (Development|PrintString "идет домой")
            (AI|AIMoveTo self (Default|GetResidentReturnLocation _hometent) 0 3e+01 true
              (:OnSuccess
                (CallFunction|FinishRoutine))
              (:OnFail
                (CallFunction|AbortRoutine))))
          (:Is%20Not%20Valid
            (Development|PrintString "не идет домой")))))))

(event Custom|FinishRoutine
  (Variables|Default|SetbRoutineRunning false))

(event Custom|Spawn4RawFishAtHole
  (params (Hole :type BP%20Water%20Source%20Ice%20Hole%20Object%20Reference))
  (Utilities|IsValid Hole
    (:Is%20Valid
      (bind _output_get (Variables|Default|SetHoleLoc (Transformation|GetActorLocation Hole)))
      (for _index (range 0 3)
        (bind _returnvalue (Game|SpawnActorfromClass :Class "/Game/BluePrints/BP_Item.BP_Item_C" :SpawnTransform (Math|Transform|MakeTransform (+ _output_get (Utilities|Array|Get(acopy) (Utilities|Array|MakeArray "0.000000,120.000000,15.000000" "120.000000,0.000000,15.000000" "-90.000000,0.000000,15.000000" "0.000000,-120.000000,15.000000") _index))) :CollisionHandlingOverride "AdjustIfPossibleButAlwaysSpawn" :TransformScaleMethod "MultiplyWithRoot" :Instigator 0))
        (Default|InitfromRowName _returnvalue "Fish_Raw")))))

(event Custom|TryStartWoodcutRoutine
  (bind _iceholemanagerref (Variables|Default|GetIceHoleManagerRef))
  (Development|PrintString "попытка лес")
  (if (not (Variables|Default|GetbRoutineRunning))
    (Utilities|IsValid _iceholemanagerref
      (:Is%20Valid
        (bind _job (Default|GetResidentJob _iceholemanagerref (Variables|Default|GetResidentRowName)))
        (if (Utilities|Enum|Equal(Enum) _job "Лесоруб")
          (bind _nearesttree (CallFunction|GetNearestFreeTree))
          (Utilities|IsValid _nearesttree
            (:Is%20Valid
              (bind _return (Default|CanbeChoppedNow _nearesttree))
              (if _return
                (Development|PrintString "ну типо норм")
                (bind _output_get (Variables|Default|SetAssignedTree _nearesttree))
                (bind _success (Default|Reserve _output_get (Variables|Default|GetResidentRowName)))
                (if _success
                  (Variables|Default|SetbRoutineRunning _success)
                  (bind _return_value (Default|GetChopLocation _output_get))
                  (AI|AIMoveTo self _return_value 0 5e+01 true
                    (:OnSuccess
                      (Development|PrintString "идет рубить")
                      (CallFunction|OnArrivedtoTree))
                    (:OnFail
                      (Development|PrintString "аборт")
                      (CallFunction|AbortWoodcutRoutine)))
                  (else
                    (Development|PrintString "ушло в false")))
                (else
                  (Development|PrintString "раньше пизда"))))
            (:Is%20Not%20Valid
              (Development|PrintString "Nearest Tree не валиден")))
          (else
            (Development|PrintString "не лесоруб")))))))

(event Custom|OnArrivedToTree
  (bind _assignedtree (Variables|Default|GetAssignedTree))
  (Utilities|IsValid _assignedtree
    (:Is%20Valid
      (Transformation|SetActorRotation (Math|Rotator|FindLookatRotation (Transformation|GetActorLocation) (Transformation|GetActorLocation _assignedtree)))
      (bind _return (Default|CanbeChoppedNow _assignedtree))
      (if _return
        (Variables|/Game/BluePrints/BP_Tree.BP_Tree_C|SetIsChopped _assignedtree true)
        (Variables|Default|SetWoodCount (Math|Random|RandomIntegerinRange 1 5))
        (bind _returnvalue (Utilities|Time|SetTimerbyEvent (delegate Custom|OnWoodcutFinished) 5.0))
        (Variables|Default|SetWoodcutTimerHandle _returnvalue)
        (else
          (Development|PrintString "ну пизда")
          (CallFunction|AbortWoodcutRoutine))))
    (:Is%20Not%20Valid
      (CallFunction|AbortWoodcutRoutine))))

(event Custom|OnWoodcutFinished
  (bind _hometent (Variables|Default|GetHomeTent))
  (Utilities|IsValid (Variables|Default|GetAssignedTree)
    (:Is%20Valid
      (if (> (Variables|Default|GetWoodCount) 0)
        (Default|AddItem (Variables|Default|GetInventoryComp) (Utilities|Struct|MakeSTR_ItemsInventory "Wood" 0 0 false (Variables|Default|GetWoodCount)))
        (Default|Release (Variables|Default|GetAssignedTree) (Variables|Default|GetResidentRowName))
        (Actor|DestroyActor (Variables|Default|GetAssignedTree))
        (Variables|Default|SetAssignedTree 0)
        (Utilities|IsValid _hometent
          (:Is%20Valid
            (Development|PrintString "идет домой")
            (AI|AIMoveTo self (Default|GetResidentReturnLocation _hometent) 0 3e+01 true
              (:OnSuccess
                (CallFunction|FinishRoutine))
              (:OnFail
                (CallFunction|AbortWoodcutRoutine))))
          (:Is%20Not%20Valid
            (Development|PrintString "не идет домой")))
        (else
          (Development|PrintString "fale у count"))))
    (:Is%20Not%20Valid
      (Development|PrintString "assigned tree не валиден"))))

(event Custom|Spawn4ItemsAtTree
  (params (Tree :type BP%20Tree%20Object%20Reference))
  (Utilities|IsValid Tree
    (:Is%20Valid
      (bind _return_value (Default|GetChopLocation Tree))
      (for _index (range 0 3)
        (bind _returnvalue (Game|SpawnActorfromClass :Class "/Game/BluePrints/BP_Item.BP_Item_C" :SpawnTransform (Math|Transform|MakeTransform (+ _return_value (Utilities|Array|Get(acopy) (Utilities|Array|MakeArray "0.000000,120.000000,0.000000" "120.000000,0.000000,0.000000" "-90.000000,0.000000,0.000000" "0.000000,-120.000000,0.000000") _index))) :CollisionHandlingOverride "AdjustIfPossibleButAlwaysSpawn" :TransformScaleMethod "MultiplyWithRoot" :Instigator 0))
        (Default|InitfromRowName _returnvalue "Wood")))))

(event EventBeginPlay
  (bind _residentdata (Variables|Default|GetResidentData))
  (bind _mesh (Variables|Character|GetMesh))
  (bind (_displayname _portrait _npcclass _skeletalmesh _animbp) (Utilities|Struct|BreakSTR_ResidentCard _residentdata))
  (Components|SkeletalMesh|SetSkeletalMeshAsset _mesh _skeletalmesh)
  (Components|SkeletalMesh|SetAnimInstanceClass _mesh _animbp)
  (bind _aswbp_npc_progress_hungry (Utilities|Casting|CastToWBP_NPC_ProgressHungry (UserInterface|GetUserWidgetObject (Variables|Default|GetWC_HungerBar)))
    (:then
      (bind _output_get (Variables|Default|SetHungerWidgetRef _aswbp_npc_progress_hungry))
      (Variables|/Game/WidgetBlueprints/WBP_NPC_ProgressHungry.WBP_NPC_ProgressHungry_C|SetOwnerNPC _output_get self)
      (Default|UpdateHungerBar _output_get)
      (Utilities|Time|SetTimerbyEvent (delegate Custom|DrainHunger) (Variables|Default|GetHungerTickInterval) true)
      (bind _outactors (Actor|GetAllActorsOfClass "/Game/BluePrints/Resources/BP_IceHoleManager.BP_IceHoleManager_C"))
      (bind _output_get_2 (Variables|Default|SetIceHoleManagerRef (Utilities|Array|Get(acopy) _outactors)))
      (EventDispatchers|BindEventtoOnResidentJobChanged _output_get_2 (delegate Custom|job)))
    (:CastFailed
      (Development|PrintString "каст не раб"))))

(event Collision|EventActorBeginOverlap
  (params (OtherActor :type Actor%20Object%20Reference)))

(event EventTick
  (params (DeltaSeconds :type Float%20%28single-precision%29)))

(fn ConstructionScript)

(fn GetNearestFreeTree
  (LocalVariables|SetBestTree 0)
  (LocalVariables|SetBestDist 99999999.0)
  (Variables|Default|SetSelfLoc (Transformation|GetActorLocation))
  (bind _outactors (Actor|GetAllActorsOfClass "/Game/BluePrints/BP_Tree.BP_Tree_C"))
  (for _array_element _outactors
    (bind _asbp_tree (Utilities|Casting|CastToBP_Tree _array_element))
    (bind _return (Default|CanbeChoppedNow _asbp_tree))
    (if _return
      (bind _return_2 (Default|IsFree _asbp_tree))
      (if _return_2
        (bind _return_value (Default|GetChopLocation _asbp_tree))
        (if (< (Math|Vector|VectorLength (- _return_value (Variables|Default|GetSelfLoc))) (LocalVariables|GetBestDist))
          (LocalVariables|SetBestDist (Math|Vector|VectorLength (- _return_value (Variables|Default|GetSelfLoc))))
          (bind _output_get (LocalVariables|SetBestTree _asbp_tree))))))
  (return _output_get))

(fn FeedNPC
  (params (FishCount :type Integer))
  (if (<= FishCount 0)
    (return 0)
    (else
      (bind _output_get (Variables|Default|SetMissingHunger (Variables|Default|GetHunger)))
      (if (<= _output_get 0.0)
        (return 0)
        (else
          (bind _output_get_2 (Variables|Default|SetNeedFish (/ (Variables|Default|GetMissingHunger) (Variables|Default|GetFeedAmountPerFish))))
          (bind _output_get_3 (LocalVariables|SetAcceptedFishCountLocal (Math|Integer|Min(Integer) (Math|Float|Ceil _output_get_2) FishCount)))
          (if (<= _output_get_3 0)
            (return 0)
            (else
              (Variables|Default|SetHunger (Math|Float|Clamp(Float) (+ (Variables|Default|GetHunger) (* _output_get_3 (Variables|Default|GetFeedAmountPerFish)))))
              (return _output_get_3))))))))

(fn GetLootData
  (bind _residentdata (Variables|Default|GetResidentData))
  (bind (_displayname _portrait) (Utilities|Struct|BreakSTR_ResidentCard _residentdata))
  (return _displayname _portrait (Variables|Default|GetWoodCount) (Variables|Default|GetFishCount)))

(fn TakeLoot
  (params (TakeWood :type Integer) (TakeFish :type Integer) (TakeFood :type Integer))
  (Variables|Default|SetTempGivenWood (Math|Integer|Clamp(Integer) TakeWood 0 (Variables|Default|GetWoodCount)))
  (Variables|Default|SetWoodCount (- (Variables|Default|GetWoodCount) (Variables|Default|GetTempGivenWood)))
  (Variables|Default|SetTempGivenFish (Math|Integer|Clamp(Integer) TakeFish 0 (Variables|Default|GetFishCount)))
  (Variables|Default|SetFishCount (- (Variables|Default|GetFishCount) (Variables|Default|GetTempGivenFish)))
  (LocalVariables|SetTemp%20Given%20Food (Math|Integer|Clamp(Integer) TakeFood 0 (Variables|Default|GetFoodCount)))
  (Variables|Default|SetFoodCount (- (Variables|Default|GetFoodCount) (LocalVariables|GetTemp%20Given%20Food)))
  (return (Variables|Default|GetTempGivenWood) (Variables|Default|GetTempGivenFish) (LocalVariables|GetTemp%20Given%20Food)))