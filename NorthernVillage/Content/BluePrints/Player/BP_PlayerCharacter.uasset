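; Player character for a snowy survival game, with walk, sprint, jump, mouse look and timed footstep sounds.
; Jumping and sprinting run looping timers that raise hunger and thirst in BPSlidersComponent and suspend its cold state until release.
; HeatField overlaps clear cold near built fires and flag trees as choppable, while capsule overlaps track the player's tent.
; A Timeline swings HoldPoint for axe chopping, and Sleep briefly disables input.
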(event OnComponentBeginOverlap(HeatField)
  (params (OverlappedComponent :type Primitive%20Component%20Object%20Reference) (OtherActor :type Actor%20Object%20Reference) (OtherComp :type Primitive%20Component%20Object%20Reference) (OtherBodyIndex :type Integer) (bFromSweep :type Boolean) (SweepResult :type Hit%20Result%20Structure%20%28by%20ref%29))
  (bind _asbp_fire (Utilities|Casting|CastToBP_Fire OtherActor)
    (:then
      (if (Variables|/Game/BluePrints/Building/BP_Build.BP_Build_C|GetisBuilt _asbp_fire)
        (Variables|/Game/BluePrints/Player/BP_SlidersComponent.BP_SlidersComponent_C|SetisCold (Variables|Default|GetBP_SlidersComponent) false)))
    (:CastFailed
      (bind _asbp_tree (Utilities|Casting|CastToBP_Tree OtherActor))
      (Variables|Default|SetisHoldTree _asbp_tree)
      (Variables|Default|SetCanChop true))))

(event OnComponentEndOverlap(HeatField)
  (params (OverlappedComponent :type Primitive%20Component%20Object%20Reference) (OtherActor :type Actor%20Object%20Reference) (OtherComp :type Primitive%20Component%20Object%20Reference) (OtherBodyIndex :type Integer))
  (Utilities|Casting|CastToBP_Fire OtherActor
    (:then
      (Variables|/Game/BluePrints/Player/BP_SlidersComponent.BP_SlidersComponent_C|SetisCold (Variables|Default|GetBP_SlidersComponent) true))
    (:CastFailed
      (bind _asbp_tree (Utilities|Casting|CastToBP_Tree OtherActor))
      (Variables|Default|SetisHoldTree _asbp_tree)
      (Variables|Default|SetCanChop false))))

(event OnComponentBeginOverlap(CapsuleComponent)
  (params (OverlappedComponent :type Primitive%20Component%20Object%20Reference) (OtherActor :type Actor%20Object%20Reference) (OtherComp :type Primitive%20Component%20Object%20Reference) (OtherBodyIndex :type Integer) (bFromSweep :type Boolean) (SweepResult :type Hit%20Result%20Structure%20%28by%20ref%29))
  (bind _asbp_player_tent (Utilities|Casting|CastToBP_PlayerTent OtherActor))
  (Variables|Default|SetPlayer%20Tent _asbp_player_tent))

(event OnComponentEndOverlap(CapsuleComponent)
  (params (OverlappedComponent :type Primitive%20Component%20Object%20Reference) (OtherActor :type Actor%20Object%20Reference) (OtherComp :type Primitive%20Component%20Object%20Reference) (OtherBodyIndex :type Integer))
  (Utilities|Casting|CastToBP_PlayerTent OtherActor)
  (Variables|Default|SetPlayer%20Tent 0))

(event Custom|Sleep
  (bind _returnvalue (Game|GetPlayerController 0))
  (Input|DisableInput _returnvalue)
  (Utilities|FlowControl|Delay 4.0)
  (Input|EnableInput _returnvalue))

(event Custom|CheckWalking
  (if (> (Math|Vector|VectorLength (Variables|/Script/Engine.MovementComponent|GetVelocity (Variables|Character|GetCharacterMovement))) 1e+01)
    (if (not (Variables|Default|GetisJump))
      (Audio|PlaySound2D "/Game/Assets/Audio/SoundCue/WalkSnowCue.WalkSnowCue" 1.0 1.0 0.0 0 0))))

(event Custom|StartAnimChop
  (Variables|Default|SetStartAxeRot "-0.000000,-100.000000,0.000000")
  (Variables|Default|SetEndAxeRot "70.000000,-100.000000,100.000000")
  (bind _alpha (Timeline|Timeline Play)
    (:Update
      (Transformation|SetRelativeRotation (Variables|Default|GetHoldPoint) (Math|Rotator|Lerp(Rotator) (Variables|Default|GetStartAxeRot) (Variables|Default|GetEndAxeRot) _alpha) false false))
    (:Finished
      (Transformation|SetRelativeRotation (Variables|Default|GetHoldPoint) (Variables|Default|GetStartAxeRot) false false))))

(event Custom|StopAnimChop
  (bind _alpha (Timeline|Timeline Stop)
    (:Update
      (Transformation|SetRelativeRotation (Variables|Default|GetHoldPoint) (Math|Rotator|Lerp(Rotator) (Variables|Default|GetStartAxeRot) (Variables|Default|GetEndAxeRot) _alpha) false false))
    (:Finished
      (Transformation|SetRelativeRotation (Variables|Default|GetHoldPoint) (Variables|Default|GetStartAxeRot) false false))))

(event Custom|Hunger
  (Default|IncreasedHunger (Variables|Default|GetBP_SlidersComponent)))

(event Custom|Thirst
  (Default|IncreasedThirst (Variables|Default|GetBP_SlidersComponent)))

(event Custom|Start
  (bind _returnvalue (Utilities|Time|SetTimerbyEvent (delegate Custom|Hunger) 0.5 true))
  (Variables|Default|SetTimerHunger _returnvalue)
  (Variables|/Game/BluePrints/Player/BP_SlidersComponent.BP_SlidersComponent_C|SetisCold (Variables|Default|GetBP_SlidersComponent) false)
  (bind _returnvalue_2 (Utilities|Time|SetTimerbyEvent (delegate Custom|Thirst) 0.25 true))
  (Variables|Default|SetTimerThirst _returnvalue_2))

(event EventBeginPlay
  (Variables|Default|SetisJump false)
  (Variables|Default|SetisRotateCamera true)
  (Variables|Default|SetCanChop false)
  (bind _output_get (Variables|Default|SetSpeedWalk 5e+02))
  (Variables|/Script/Engine.CharacterMovementComponent|SetMaxWalkSpeed (Variables|Character|GetCharacterMovement) _output_get)
  (Variables|Default|SetSpeedSprint 1e+03)
  (Utilities|Time|SetTimerbyEvent (delegate Custom|CheckWalking) 0.5 true)
  (Default|StartGame (Variables|Default|GetBP_InventoryComponent))
  (Default|StartGame (Variables|Default|GetBP_SlidersComponent))
  (Variables|Default|SetisCanSleep false))

(event Collision|EventActorBeginOverlap
  (params (OtherActor :type Actor%20Object%20Reference)))

(event EventTick
  (params (DeltaSeconds :type Float%20%28single-precision%29)))

(event Input|ActionEvents|InputActionJump
  (params (Key :type Key%20Structure :default "None"))
  (:Pressed
    (Character|Jump)
    (CallFunction|Start)
    (Variables|Default|SetisJump true)
    (Audio|PlaySound2D "/Game/Assets/Audio/SoundCue/WalkSnowCue.WalkSnowCue" 1.0 1.0 0.0 0 0))
  (:Released
    (Character|StopJumping)
    (Utilities|FlowControl|Delay 1.0)
    (Utilities|Time|ClearandInvalidateTimerbyHandle (Variables|Default|GetTimerHunger))
    (Variables|/Game/BluePrints/Player/BP_SlidersComponent.BP_SlidersComponent_C|SetisCold (Variables|Default|GetBP_SlidersComponent) true)
    (Variables|Default|SetisJump false)
    (Utilities|Time|ClearandInvalidateTimerbyHandle (Variables|Default|GetTimerThirst))
    (Audio|PlaySound2D "/Game/Assets/Audio/SoundCue/WalkSnowCue.WalkSnowCue" 1.0 1.0 0.0 0 0)))

(event Input|ActionEvents|InputActionSprint
  (params (Key :type Key%20Structure :default "None"))
  (bind _charactermovement (Variables|Character|GetCharacterMovement))
  (:Pressed
    (Variables|/Script/Engine.CharacterMovementComponent|SetMaxWalkSpeed _charactermovement (Variables|Default|GetSpeedSprint))
    (CallFunction|Start))
  (:Released
    (Variables|/Script/Engine.CharacterMovementComponent|SetMaxWalkSpeed _charactermovement (Variables|Default|GetSpeedWalk))
    (Utilities|Time|ClearandInvalidateTimerbyHandle (Variables|Default|GetTimerHunger))
    (Variables|/Game/BluePrints/Player/BP_SlidersComponent.BP_SlidersComponent_C|SetisCold (Variables|Default|GetBP_SlidersComponent) true)
    (Utilities|Time|ClearandInvalidateTimerbyHandle (Variables|Default|GetTimerThirst))))

(event Input|AxisEvents|InputAxisMoveForward
  (params (AxisValue :type Float%20%28single-precision%29))
  ;[0.15 0.15 0.15 0.5] WASD Controll
  (Pawn|Input|AddMovementInput (Transformation|GetActorForwardVector (Game|GetPlayerCharacter 0)) AxisValue false))

(event Input|AxisEvents|InputAxisMoveRight
  (params (AxisValue :type Float%20%28single-precision%29))
  ;[0.15 0.15 0.15 0.5] WASD Controll
  (Pawn|Input|AddMovementInput (Transformation|GetActorRightVector (Game|GetPlayerCharacter 0)) AxisValue false))

(event Input|AxisEvents|InputAxisTurn
  (params (AxisValue :type Float%20%28single-precision%29))
  ;[0.15 0.15 0.15 0.5] Camera
  (if (Variables|Default|GetisRotateCamera)
    (Pawn|Input|AddControllerYawInput AxisValue)))

(event Input|AxisEvents|InputAxisLookUp
  (params (AxisValue :type Float%20%28single-precision%29))
  ;[0.15 0.15 0.15 0.5] Camera
  (if (Variables|Default|GetisRotateCamera)
    (Pawn|Input|AddControllerPitchInput AxisValue)))

(fn ConstructionScript)