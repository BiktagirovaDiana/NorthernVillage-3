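; Player survival component that tracks cold, hunger and thirst and drives their HUD sliders in WBPSliders.
; Looping timers drain each stat, with cooling faster at night based on the SunMoonDaySequenceActor clock, and warmth recovering while IsCold is false.
; Eat and Drink refill stats with side effects on thirst and heat, while low warmth fades in a frost overlay.
; Any stat reaching zero calls Lose, which pauses the game and shows WBP_Lose.
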(event Custom|Freez
  (if (Variables|Default|GetisCold)
    (if (<= (Variables|Default|GetCold) 0.0)
      (CallFunction|Lose)
      (else
        (Variables|Default|SetCold (- (Variables|Default|GetCold) (Variables|Default|GetLevelFreez)))
        (if (< (Variables|Default|GetCold) 5e+01)
          (Class|Image|SetBrushTintColor (Variables|/Game/WidgetBlueprints/WBP_Sliders.WBP_Sliders_C|GetImageFrost (Variables|Default|GetWBP:_Sliders)) (Utilities|Struct|MakeSlateColor (Utilities|Struct|MakeLinearColor 1.0 1.0 1.0 (Math|Float|MapRangeClamped (Variables|Default|GetCold) 0.0 5e+01 1.0 0.0)) "UseColor_Specified")))))
    (elif (not (>= (Variables|Default|GetCold) 1e+02))
      (bind _output_get (Variables|Default|SetCold (+ (Variables|Default|GetCold) 3.0)))
      (Default|SetPercentHeat (Variables|Default|GetWBP:_Sliders) (Utilities|100to1 _output_get))
      (Class|Image|SetBrushTintColor (Variables|/Game/WidgetBlueprints/WBP_Sliders.WBP_Sliders_C|GetImageFrost (Variables|Default|GetWBP:_Sliders)) (Utilities|Struct|MakeSlateColor (Utilities|Struct|MakeLinearColor 1.0 1.0 1.0 (Math|Float|MapRangeClamped (Variables|Default|GetCold) 0.0 5e+01 1.0 0.0)) "UseColor_Specified")))))

(event Custom|Start
  (bind _returnvalue (Utilities|Time|SetTimerbyEvent (delegate Custom|Freez) 1.0 true))
  (Variables|Default|SetFreezeTimer _returnvalue)
  (bind _returnvalue_2 (Utilities|Time|SetTimerbyEvent (delegate Custom|IncreasedThirst) 3.0 true))
  (Variables|Default|SetThirstTimer _returnvalue_2)
  (bind _returnvalue_3 (Utilities|Time|SetTimerbyEvent (delegate Custom|IncreasedHunger) 5.0 true))
  (Variables|Default|SetHungerTimer _returnvalue_3))

(event Custom|Eat
  (params (Satiety :type Float%20%28double-precision%29))
  (if (< 1e+02 (+ Satiety (Variables|Default|GetHunger)))
    (bind _output_get (Variables|Default|SetHunger 1e+02))
    (Default|SetPercentHunger (Variables|Default|GetWBP:_Sliders) (Utilities|100to1 _output_get))
    (else
      (bind _output_get_2 (Variables|Default|SetHunger (+ Satiety (Variables|Default|GetHunger))))
      (Default|SetPercentHunger (Variables|Default|GetWBP:_Sliders) (Utilities|100to1 _output_get_2))))
  (bind _output_get_3 (Variables|Default|SetThirst (- (Variables|Default|GetThirst) (Math|Float|%(Float) Satiety 25.0))))
  (Default|SetPercentThirst (Variables|Default|GetWBP:_Sliders) (Utilities|100to1 _output_get_3)))

(event Custom|Lose
  (Utilities|Time|ClearandInvalidateTimerbyHandle (Variables|Default|GetHungerTimer))
  (Utilities|Time|ClearandInvalidateTimerbyHandle (Variables|Default|GetThirstTimer))
  (Utilities|Time|ClearandInvalidateTimerbyHandle (Variables|Default|GetFreezeTimer))
  (bind _returnvalue (UserInterface|CreateWidget "/Game/WidgetBlueprints/WBP_Lose.WBP_Lose_C"))
  (UserInterface|Viewport|AddtoViewport _returnvalue 0)
  (Game|SetGamePaused true)
  (Variables|/Script/Engine.PlayerController|SetbShowMouseCursor (Variables|Default|GetBP%20Player%20Controller) true))

(event Custom|Drink
  (params (Water :type Float%20%28double-precision%29) (isColdWater :type Boolean))
  (if (< 1e+02 (+ Water (Variables|Default|GetThirst)))
    (bind _output_get (Variables|Default|SetThirst 1e+02))
    (Default|SetPercentThirst (Variables|Default|GetWBP:_Sliders) (Utilities|100to1 _output_get))
    (else
      (bind _output_get_2 (Variables|Default|SetThirst (+ Water (Variables|Default|GetThirst))))
      (Default|SetPercentThirst (Variables|Default|GetWBP:_Sliders) (Utilities|100to1 _output_get_2))))
  (if isColdWater
    (if (>= (- (Variables|Default|GetCold) 25.0) 1e+02)
      (bind _output_get_3 (Variables|Default|SetCold 9e+01))
      (Default|SetPercentHeat (Variables|Default|GetWBP:_Sliders) (Utilities|100to1 _output_get_3))
      (else
        (bind _output_get_4 (Variables|Default|SetCold (- (Variables|Default|GetCold) 25.0)))
        (Default|SetPercentHeat (Variables|Default|GetWBP:_Sliders) (Utilities|100to1 _output_get_4))))))

(event Custom|CheckTime
  (bind _sunmoondayactor (Variables|Default|GetSunMoonDayActor))
  (bind _returnvalue (Class|DaySequenceActor|GetTimeOfDay _sunmoondayactor))
  (bind _returnvalue_2 (Math|Float|Floor _returnvalue))
  (if (and (> _returnvalue_2 6) (< _returnvalue_2 18))
    (Variables|Default|SetLevelFreez 1.0)
    (Class|Image|SetBrushTintColor (Variables|/Game/WidgetBlueprints/WBP_Sliders.WBP_Sliders_C|GetHeatFull (Variables|Default|GetWBP:_Sliders)) (Utilities|Struct|MakeSlateColor "(R=1.000000,G=0.194618,B=0.029557,A=1.000000)"))
    (else
      (Variables|Default|SetLevelFreez 3.0)
      (Class|Image|SetBrushTintColor (Variables|/Game/WidgetBlueprints/WBP_Sliders.WBP_Sliders_C|GetHeatFull (Variables|Default|GetWBP:_Sliders)) (Utilities|Struct|MakeSlateColor "(R=0.003798,G=0.038610,B=0.104167,A=1.000000)")))))

(event Custom|IncreasedHunger
  (if (<= (Variables|Default|GetHunger) 0.0)
    (CallFunction|Lose)
    (else
      (bind _output_get (Variables|Default|SetHunger (- (Variables|Default|GetHunger) 1.0)))
      (Default|SetPercentHunger (Variables|Default|GetWBP:_Sliders) (Utilities|100to1 _output_get)))))

(event Custom|IncreasedThirst
  (if (<= (Variables|Default|GetThirst) 0.0)
    (CallFunction|Lose)
    (else
      (bind _output_get (Variables|Default|SetThirst (- (Variables|Default|GetThirst) 1.0)))
      (Default|SetPercentThirst (Variables|Default|GetWBP:_Sliders) (Utilities|100to1 _output_get)))))

(event EventBeginPlay
  (Utilities|FlowControl|Delay 1.0)
  (bind _asbp_game_mode (Utilities|Casting|CastToBP_GameMode (Game|GetGameMode)))
  (Variables|Default|SetWBP:_Sliders (Variables|/Game/BluePrints/BP_GameMode.BP_GameMode_C|GetWBP%20Sliders _asbp_game_mode))
  (Variables|Default|SetLevelFreez 1.0)
  (Utilities|Time|SetTimerbyEvent (delegate Custom|CheckTime) 5.0 true)
  (Variables|Default|SetCold 1e+02)
  (Variables|Default|SetHunger 1e+02)
  (Variables|Default|SetThirst 1e+02)
  (Variables|Default|SetisCold true)
  (CallFunction|Start)
  (bind _outactors (Actor|GetAllActorsOfClass "/Script/DaySequence.SunMoonDaySequenceActor"))
  (for _array_element _outactors
    (Variables|Default|SetSunMoonDayActor _array_element))
  (Class|Image|SetBrushTintColor (Variables|/Game/WidgetBlueprints/WBP_Sliders.WBP_Sliders_C|GetImageFrost (Variables|Default|GetWBP:_Sliders)) (Utilities|Struct|MakeSlateColor (Utilities|Struct|MakeLinearColor 1.0 1.0 1.0 0.0) "UseColor_Specified"))
  (bind _asbp_player_controller (Utilities|Casting|CastToBP_PlayerController (Game|GetPlayerController 0)))
  (Variables|Default|SetBP%20Player%20Controller _asbp_player_controller))

(event EventTick
  (params (DeltaSeconds :type Float%20%28single-precision%29)))