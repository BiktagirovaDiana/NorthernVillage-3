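; Player component that turns input into survival actions: villager inventory, item use, building, eating, drinking and sleeping.
; Interact opens the current NPC's inventory or acts on the held item: filling containers, fishing, chopping, crafting torches.
; Looping timers drive hold-to-fish, chopping and trace-based build placement, which updates GameMode tasks and shows the win screen at five tents.
; Items come from DT_ItemsInventor; sleep requires night and a fire-warmed tent.
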(event Custom|Chop
  (bind (_start _end) (Utilities|TraceLocations))
  (bind _outhit (Collision|LineTraceByChannel _start _end "TraceTypeQuery1" false 0 "None"))
  (bind _asbp_tree (Utilities|Casting|CastToBP_Tree (.hitactor _outhit))
    (:then
      (Default|StartAnimChop (Variables|Default|GetPlayerCharacter))
      (if (Variables|Default|GetisHoldingKey)
        (Default|AnimChopTree _asbp_tree)
        (bind _output_get (Variables|Default|SetTime (+ (Variables|Default|GetTime) 0.5)))
        (Default|UpdateBar2 (Variables|Default|GetWBP_ProgressFishing) 5.0 _output_get)
        (Audio|PlaySound2D "/Game/Assets/Audio/SoundCue/TreeChopCue.TreeChopCue" 1.0 1.0 0.0 0 0)
        (if (>= (Variables|Default|GetTime) 5.0)
          (bind _returnvalue (Utilities|GetDataTableRow "/Game/BluePrints/Resources/DT_ItemsInventor.DT_ItemsInventor" "Wood")
            (:then
              (Default|AddItem (Variables|/Game/BluePrints/Player/BP_PlayerCharacter.BP_PlayerCharacter_C|GetBP_InventoryComponent (Variables|Default|GetPlayerCharacter)) (Utilities|Struct|MakeSTR_ItemsInventory (.name _returnvalue) (.icon _returnvalue) (.mesh _returnvalue) (.stackabled _returnvalue) (Math|Random|RandomIntegerinRange 3 8) (.maxstackebled _returnvalue) (.scale _returnvalue) (.enum _returnvalue) (.location _returnvalue) (.rotation _returnvalue)))
              (Variables|Default|SetTime 0.0)
              (Utilities|IsValid 0
                (:Is%20Valid
                  (Variables|/Game/BluePrints/BP_Tree.BP_Tree_C|SetIsChopped _asbp_tree true)
                  (Variables|/Game/BluePrints/BP_Tree.BP_Tree_C|SetbReserved _asbp_tree true)
                  (Actor|DestroyActor _asbp_tree)
                  (Widget|SetVisibility (Variables|Default|GetWBP_ProgressFishing) "Hidden"))
                (:Is%20Not%20Valid
                  (Actor|DestroyActor _asbp_tree)
                  (Widget|SetVisibility (Variables|Default|GetWBP_ProgressFishing) "Hidden"))))))
        (else
          (bind _output_get_2 (Variables|Default|SetTime 0.0 :!label _label))
          (Default|UpdateBar2 (Variables|Default|GetWBP_ProgressFishing) 5.0 _output_get_2)
          (Widget|SetVisibility (Variables|Default|GetWBP_ProgressFishing) "Hidden")
          (Utilities|Time|ClearandInvalidateTimerbyHandle (Variables|Default|GetChopTimer))
          (Default|StopAnimChop (Variables|Default|GetPlayerCharacter)))))
    (:CastFailed
      (goto _label))))

(event Custom|OnFishCaught
  (bind _playercharacter (Variables|Default|GetPlayerCharacter))
  (if (Variables|Default|GetisHoldingKey)
    (if (Variables|/Game/BluePrints/Player/BP_PlayerCharacter.BP_PlayerCharacter_C|GetIsFishing _playercharacter)
      (if (Variables|/Game/BluePrints/Player/BP_PlayerCharacter.BP_PlayerCharacter_C|GetCanFish _playercharacter)
        (bind _output_get (Variables|Default|SetTime (+ (Variables|Default|GetTime) 0.25)))
        (Default|UpdateBar2 (Variables|Default|GetWBP_ProgressFishing) (Variables|Default|GetTimer) _output_get)
        (if (>= (Variables|Default|GetTime) (Variables|Default|GetTimer))
          (bind _returnvalue (Utilities|GetDataTableRow "/Game/BluePrints/Resources/DT_ItemsInventor.DT_ItemsInventor" "Raw_Fish")
            (:then
              (Default|AddItem (Variables|/Game/BluePrints/Player/BP_PlayerCharacter.BP_PlayerCharacter_C|GetBP_InventoryComponent (Variables|Default|GetPlayerCharacter)) (Utilities|Struct|MakeSTR_ItemsInventory (.name _returnvalue) (.icon _returnvalue) (.mesh _returnvalue) (.stackabled _returnvalue) (.quanity _returnvalue) (.maxstackebled _returnvalue) (.scale _returnvalue) (.enum _returnvalue) (.location _returnvalue) (.rotation _returnvalue)))
              (Variables|/Game/BluePrints/Player/BP_PlayerCharacter.BP_PlayerCharacter_C|SetIsFishing (Variables|Default|GetPlayerCharacter) false))))
        (else
          (Widget|SetVisibility (Variables|Default|GetWBP_ProgressFishing) "Hidden")))
      (else
        (Widget|SetVisibility (Variables|Default|GetWBP_ProgressFishing) "Hidden")))
    (else
      (bind _output_get_2 (Variables|Default|SetTime 0.0))
      (Default|UpdateBar2 (Variables|Default|GetWBP_ProgressFishing) (Variables|Default|GetTimer) _output_get_2)
      (Widget|SetVisibility (Variables|Default|GetWBP_ProgressFishing) "Hidden")
      (Utilities|Time|ClearandInvalidateTimerbyHandle (Variables|Default|GetFishingTimerHandle))
      (Audio|SpawnSound2D "/Game/Assets/Audio/Sounds/FishingRod3.FishingRod3" 1.0 1.0 0.0 0))))

(event Custom|ChangeLocation
  (bind (_start _end) (Utilities|TraceLocations))
  (bind _gamemode (Variables|Default|GetGameMode))
  (bind _gamemode_2 (Variables|Default|GetGameMode))
  ;[0.15 0.15 0.15 0.5] Change Location Build
  (if (Variables|Default|GetisChangeLocation)
    (bind _outhit (Collision|LineTraceByChannel _start _end "TraceTypeQuery1" false 0 "None"))
    (Utilities|Casting|CastToLandscape (.HitActor (Collision|BreakHitResult _outhit)))
    (Transformation|SetActorLocation (Variables|Default|GetHoldBuild) (.ImpactPoint (Collision|BreakHitResult _outhit)) false false)
    (else
      (Utilities|Time|ClearandInvalidateTimerbyHandle (Variables|Default|GetTimerBuilding))
      (bind _asbp_fire (Utilities|Casting|CastToBP_Fire (Variables|Default|GetHoldBuild))
        (:then
          (Default|CheckPlayer _asbp_fire)
          (Variables|Default|SetHoldBuild 0))
        (:CastFailed
          (bind _asbp_player_tent (Utilities|Casting|CastToBP_PlayerTent (Variables|Default|GetHoldBuild))
            (:then
              (Variables|/Game/BluePrints/Building/BP_Build.BP_Build_C|SetisBuilt (Variables|/Game/BluePrints/Building/BP_PlayerTent.BP_PlayerTent_C|Get%20BP%20Fire _asbp_player_tent) true))
            (:CastFailed
              _))))
      (Audio|PlaySound2D "/Game/Assets/Audio/SoundCue/HammerCue.HammerCue" 1.0 1.0 0.0 0 0)
      (Variables|Default|SetisRotateBuild false)
      (Collision|SetCollisionEnabled (Variables|/Game/BluePrints/Building/BP_Build.BP_Build_C|GetMesh1 (Variables|Default|GetHoldBuild)) "QueryAndPhysics")
      (Collision|SetCollisionEnabled (Variables|/Game/BluePrints/Building/BP_Build.BP_Build_C|GetMesh2 (Variables|Default|GetHoldBuild)) "QueryAndPhysics")
      (Utilities|Casting|CastToBP_Tent (Variables|Default|GetHoldBuild)
        (:then
          (switch Utilities|FlowControl|Switch|SwitchonENUM_TaskBuild (Variables|/Game/BluePrints/BP_GameMode.BP_GameMode_C|GetTaskBuild _gamemode)
            (:NewEnumerator2
              _)
            (:NewEnumerator0
              (Variables|/Game/BluePrints/BP_GameMode.BP_GameMode_C|SetisTaskBuild _gamemode true))
            (:NewEnumerator1
              _))
          (Collision|SetCollisionEnabled (Variables|/Game/BluePrints/Building/BP_Build.BP_Build_C|GetMesh1 (Variables|Default|GetHoldBuild)) "QueryAndPhysics")
          (Collision|SetCollisionEnabled (Variables|/Game/BluePrints/Building/BP_Build.BP_Build_C|GetMesh2 (Variables|Default|GetHoldBuild)) "QueryAndPhysics"))
        (:CastFailed
          (Utilities|Casting|CastToBP_Tent (Variables|Default|GetHoldBuild))
          (switch Utilities|FlowControl|Switch|SwitchonENUM_TaskBuild (Variables|/Game/BluePrints/BP_GameMode.BP_GameMode_C|GetTaskBuild _gamemode_2)
            (:NewEnumerator2
              _)
            (:NewEnumerator0
              _)
            (:NewEnumerator1
              (Variables|/Game/BluePrints/BP_GameMode.BP_GameMode_C|SetisTaskBuild _gamemode_2 true)))))
      (Variables|Default|SetNumberBuilds 0)
      (bind _outactors (Actor|GetAllActorsOfClass "/Game/BluePrints/Building/BP_Tent.BP_Tent_C"))
      (for _array_element _outactors
        (Variables|Default|SetNumberBuilds (+ (Variables|Default|GetNumberBuilds) 1)))
      (if (>= (Variables|Default|GetNumberBuilds) 5)
        (bind _returnvalue (UserInterface|CreateWidget "/Game/WidgetBlueprints/WBP_Win.WBP_Win_C"))
        (UserInterface|Viewport|AddtoViewport _returnvalue 0)
        (Game|SetGamePaused true)))))

(event Custom|Building
  (params (BP_Build :type BP%20Build%20Class%20Reference))
  (bind (_start _end) (Utilities|TraceLocations))
  ;[0.15 0.15 0.15 0.5] Change Location Build
  (bind (_outhit _returnvalue) (Collision|LineTraceByChannel _start _end "TraceTypeQuery1" false 0 "None"))
  (if _returnvalue
    (bind _returnvalue_2 (Game|SpawnActorfromClass BP_Build (Math|Conversions|ToTransform(Vector) (.ImpactPoint (Collision|BreakHitResult _outhit))) "AdjustIfPossibleButAlwaysSpawn" "MultiplyWithRoot" 0 false 0))
    (bind _output_get (Variables|Default|SetHoldBuild _returnvalue_2))
    (Utilities|IsValid _output_get
      (:Is%20Valid
        (Variables|/Game/BluePrints/Building/BP_Build.BP_Build_C|SetisBuilt _output_get false)
        (Default|CanBuild _output_get)
        (Variables|Default|SetisRotateBuild true)
        (Collision|SetCollisionEnabled (Variables|/Game/BluePrints/Building/BP_Build.BP_Build_C|GetMesh1 (Variables|Default|GetHoldBuild)) "NoCollision")
        (Collision|SetCollisionEnabled (Variables|/Game/BluePrints/Building/BP_Build.BP_Build_C|GetMesh2 (Variables|Default|GetHoldBuild)) "NoCollision")
        (bind _returnvalue_3 (Utilities|Time|SetTimerbyEvent (delegate Custom|ChangeLocation) (Utilities|Time|GetWorldDeltaSeconds) true))
        (Variables|Default|SetTimerBuilding _returnvalue_3)))))

(event Custom|Hint
  (params (Text :type Text) (isTime :type Boolean))
  (if isTime
    (bind _returnvalue (UserInterface|CreateWidget "/Game/WidgetBlueprints/WBP_Text.WBP_Text_C"))
    (bind _output_get (Variables|Default|SetCurrentHint _returnvalue))
    (Default|UpdateText _output_get Text)
    (UserInterface|Viewport|AddtoViewport (Variables|Default|GetCurrentHint) 0)
    (Utilities|FlowControl|Delay 0.5)
    (Widget|SetVisibility (Variables|Default|GetCurrentHint) "Hidden")
    (else
      (bind _returnvalue_2 (UserInterface|CreateWidget "/Game/WidgetBlueprints/WBP_Text.WBP_Text_C"))
      (bind _output_get_2 (Variables|Default|SetCurrentHint _returnvalue_2))
      (Default|UpdateText _output_get_2 Text)
      (UserInterface|Viewport|AddtoViewport (Variables|Default|GetCurrentHint) 0))))

(event Custom|CloseHInt
  (Widget|SetVisibility (Variables|Default|GetCurrentHint) "Hidden"))

(event EventBeginPlay
  (bind _asbp_player_character (Utilities|Casting|CastToBP_PlayerCharacter (Game|Player|GetPlayerPawn 0)))
  (Variables|Default|SetPlayerCharacter _asbp_player_character)
  (bind _asbp_player_controller (Utilities|Casting|CastToBP_PlayerController (Game|GetPlayerController 0)))
  (Variables|Default|SetPlayerController _asbp_player_controller)
  (Variables|Default|SetMaxDistanceLine 1e+03)
  (Variables|Default|SetisChangeLocation false)
  (bind _asbp_game_mode (Utilities|Casting|CastToBP_GameMode (Game|GetGameMode)))
  (Variables|Default|SetGameMode _asbp_game_mode))

(event Input|ActionEvents|InputActionInteract
  (params (Key :type Key%20Structure :default "None"))
  (bind _returnvalue (Game|GetPlayerController 0))
  (bind (_start _end) (Utilities|TraceLocations))
  (bind (_start_2 _end_2) (Utilities|TraceLocations))
  (bind _playercharacter (Variables|Default|GetPlayerCharacter))
  (bind _playercharacter_2 (Variables|Default|GetPlayerCharacter))
  (bind _playercharacter_3 (Variables|Default|GetPlayerCharacter))
  (bind _playercharacter_4 (Variables|Default|GetPlayerCharacter))
  (bind _playercharacter_5 (Variables|Default|GetPlayerCharacter))
  (bind _playercharacter_6 (Variables|Default|GetPlayerCharacter))
  (bind _bp_inventorycomponent (Variables|/Game/BluePrints/Player/BP_PlayerCharacter.BP_PlayerCharacter_C|GetBP_InventoryComponent _playercharacter))
  (bind _bp_inventorycomponent_2 (Variables|/Game/BluePrints/Player/BP_PlayerCharacter.BP_PlayerCharacter_C|GetBP_InventoryComponent _playercharacter_2))
  (bind _bp_inventorycomponent_3 (Variables|/Game/BluePrints/Player/BP_PlayerCharacter.BP_PlayerCharacter_C|GetBP_InventoryComponent _playercharacter_3))
  (bind _bp_inventorycomponent_4 (Variables|/Game/BluePrints/Player/BP_PlayerCharacter.BP_PlayerCharacter_C|GetBP_InventoryComponent _playercharacter_4))
  (bind _bp_inventorycomponent_5 (Variables|/Game/BluePrints/Player/BP_PlayerCharacter.BP_PlayerCharacter_C|GetBP_InventoryComponent _playercharacter_5))
  (bind _holditem (Variables|/Game/BluePrints/Player/BP_InventoryComponent.BP_InventoryComponent_C|GetHoldItem _bp_inventorycomponent_5))
  (:Pressed
    (Variables|Default|SetisHoldingKey true)
    (Utilities|IsValid (Variables|Default|GetCurrentInteractable)
      (:Is%20Valid
        (bind _asbp_npc_villager_base (Utilities|Casting|CastToBP_NPC_VillagerBase (Variables|Default|GetCurrentInteractable)))
        (bind _returnvalue_2 (UserInterface|CreateWidget "/Game/BluePrints/AI/WBP_NPCInventory.WBP_NPCInventory_C" _returnvalue _asbp_npc_villager_base))
        (Default|InitfromNPC _returnvalue_2 _asbp_npc_villager_base)
        (UserInterface|Viewport|AddtoViewport _returnvalue_2 0)
        (Input|SetInputModeGameandUI _returnvalue _returnvalue_2 "DoNotLock" true false)
        (Variables|/Script/Engine.PlayerController|SetbShowMouseCursor _returnvalue true)
        (Game|SetGamePaused true))
      (:Is%20Not%20Valid
        (Utilities|IsValid _holditem
          (:Is%20Valid
            (if (not (Variables|/Game/BluePrints/Player/BP_InventoryComponent.BP_InventoryComponent_C|GetisFreeHand (Variables|/Game/BluePrints/Player/BP_PlayerCharacter.BP_PlayerCharacter_C|GetBP_InventoryComponent (Variables|Default|GetPlayerCharacter))))
              (switch Utilities|FlowControl|Switch|SwitchonENUM_Item (.Enum (Utilities|Struct|BreakSTR_ItemsInventory (Variables|/Game/BluePrints/BP_Item.BP_Item_C|GetItem _holditem)))
                (:NewEnumerator1
                  (if (Variables|/Game/BluePrints/Player/BP_PlayerCharacter.BP_PlayerCharacter_C|GetCanFillWater (Variables|Default|GetPlayerCharacter))
                    (Variables|Default|SetRowName "Bucket_ColdWater3")
                    (else
                      (bind _outhit (Collision|LineTraceByChannel _start _end "TraceTypeQuery1" false 0 "None"))
                      (Utilities|Casting|CastToLandscape (.HitActor (Collision|BreakHitResult _outhit)))
                      (Variables|Default|SetRowName "Bucket_Snow")))
                  (bind _returnvalue_3 (Utilities|GetDataTableRow "/Game/BluePrints/Resources/DT_ItemsInventor.DT_ItemsInventor" (Variables|Default|GetRowName))
                    (:then
                      (bind _output_get (Variables|/Game/BluePrints/BP_Item.BP_Item_C|SetItem (Variables|/Game/BluePrints/Player/BP_InventoryComponent.BP_InventoryComponent_C|GetHoldItem (Variables|/Game/BluePrints/Player/BP_PlayerCharacter.BP_PlayerCharacter_C|GetBP_InventoryComponent (Variables|Default|GetPlayerCharacter))) (Utilities|Struct|MakeSTR_ItemsInventory (.name _returnvalue_3) (.icon _returnvalue_3) (.mesh _returnvalue_3) (.stackabled _returnvalue_3) (.quanity _returnvalue_3) (.maxstackebled _returnvalue_3) (.scale _returnvalue_3) (.enum _returnvalue_3) (.location _returnvalue_3) (.rotation _returnvalue_3))))
                      (Utilities|Array|SetArrayElem (Variables|/Game/BluePrints/Player/BP_InventoryComponent.BP_InventoryComponent_C|GetItems _bp_inventorycomponent_2) (Variables|/Game/BluePrints/Player/BP_InventoryComponent.BP_InventoryComponent_C|GetCurrentSlotIndex _bp_inventorycomponent_2) _output_get)
                      (Default|ResizeandLoad _bp_inventorycomponent_2)
                      (Actor|DestroyActor (Variables|/Game/BluePrints/Player/BP_InventoryComponent.BP_InventoryComponent_C|GetHoldItem _bp_inventorycomponent_2)))))
                (:NewEnumerator3
                  (if (Variables|/Game/BluePrints/Player/BP_PlayerCharacter.BP_PlayerCharacter_C|GetCanFish _playercharacter_6)
                    (if (not (Variables|/Game/BluePrints/Player/BP_PlayerCharacter.BP_PlayerCharacter_C|GetIsFishing _playercharacter_6))
                      (Variables|/Game/BluePrints/Player/BP_PlayerCharacter.BP_PlayerCharacter_C|SetIsFishing (Variables|Default|GetPlayerCharacter) true)
                      (bind _returnvalue_4 (UserInterface|CreateWidget "/Game/WidgetBlueprints/WBP_ProgressFishing.WBP_ProgressFishing_C"))
                      (bind _output_get_2 (Variables|Default|SetWBP_ProgressFishing _returnvalue_4))
                      (UserInterface|Viewport|AddtoViewport _output_get_2 0)
                      (bind _output_get_3 (Variables|Default|SetTimer (Math|Random|RandomFloatinRange 2.0 7.0)))
                      (Default|UpdateBar (Variables|Default|GetWBP_ProgressFishing) _output_get_3)
                      (Audio|SpawnSound2D "/Game/Assets/Audio/Sounds/FishingRod1.FishingRod1" 1.0 1.0 0.0 0)
                      (bind _returnvalue_5 (Utilities|Time|SetTimerbyEvent (delegate Custom|OnFishCaught) 0.25 true))
                      (Variables|Default|SetFishingTimerHandle _returnvalue_5))))
                (:NewEnumerator4
                  (if (Variables|/Game/BluePrints/Player/BP_PlayerCharacter.BP_PlayerCharacter_C|GetCanChop (Variables|Default|GetPlayerCharacter))
                    (bind _returnvalue_6 (UserInterface|CreateWidget "/Game/WidgetBlueprints/WBP_ProgressFishing.WBP_ProgressFishing_C"))
                    (bind _output_get_4 (Variables|Default|SetWBP_ProgressFishing _returnvalue_6))
                    (UserInterface|Viewport|AddtoViewport _output_get_4 0)
                    (bind _returnvalue_7 (Utilities|Time|SetTimerbyEvent (delegate Custom|Chop) 0.5 true))
                    (Variables|Default|SetChopTimer _returnvalue_7)
                    (else
                      (Default|StopAnimChop (Variables|Default|GetPlayerCharacter)))))
                (:NewEnumerator10
                  (bind _returnvalue_8 (Utilities|GetDataTableRow "/Game/BluePrints/Resources/DT_ItemsInventor.DT_ItemsInventor" "Torch")
                    (:then
                      (Default|RemoveItem _bp_inventorycomponent_4 (Variables|/Game/BluePrints/Player/BP_InventoryComponent.BP_InventoryComponent_C|GetCurrentSlotIndex _bp_inventorycomponent_4) 1)
                      (Default|AddItem _bp_inventorycomponent_4 (Utilities|Struct|MakeSTR_ItemsInventory (.name _returnvalue_8) (.icon _returnvalue_8) (.mesh _returnvalue_8) (.stackabled _returnvalue_8) (.quanity _returnvalue_8) (.maxstackebled _returnvalue_8) (.scale _returnvalue_8) (.enum _returnvalue_8) (.location _returnvalue_8) (.rotation _returnvalue_8)))
                      (Actor|DestroyActor (Variables|/Game/BluePrints/Player/BP_InventoryComponent.BP_InventoryComponent_C|GetHoldItem _bp_inventorycomponent_4)))))
                (:NewEnumerator12
                  (bind _outhit_2 (Collision|LineTraceByChannel _start_2 _end_2 "TraceTypeQuery1" false 0 "None"))
                  (bind _asbp_item (Utilities|Casting|CastToBP_Item (.HitActor (Collision|BreakHitResult _outhit_2))))
                  (switch Utilities|FlowControl|Switch|SwitchonENUM_Item (.Enum (Utilities|Struct|BreakSTR_ItemsInventory (Variables|/Game/BluePrints/BP_Item.BP_Item_C|GetItem _asbp_item)))
                    (:NewEnumerator6
                      (bind _returnvalue_9 (Utilities|GetDataTableRow "/Game/BluePrints/Resources/DT_ItemsInventor.DT_ItemsInventor" "Bucket_Empty")
                        (:then
                          (Default|ApplyItemData _asbp_item _returnvalue_9)
                          (bind _returnvalue_10 (Utilities|GetDataTableRow "/Game/BluePrints/Resources/DT_ItemsInventor.DT_ItemsInventor" "Flask_ColdWater" :!label _label)
                            (:then
                              (bind _output_get_5 (Variables|/Game/BluePrints/BP_Item.BP_Item_C|SetItem (Variables|/Game/BluePrints/Player/BP_InventoryComponent.BP_InventoryComponent_C|GetHoldItem (Variables|/Game/BluePrints/Player/BP_PlayerCharacter.BP_PlayerCharacter_C|GetBP_InventoryComponent (Variables|Default|GetPlayerCharacter))) (Utilities|Struct|MakeSTR_ItemsInventory (.name _returnvalue_10) (.icon _returnvalue_10) (.mesh _returnvalue_10) (.stackabled _returnvalue_10) (.quanity _returnvalue_10) (.maxstackebled _returnvalue_10) (.scale _returnvalue_10) (.enum _returnvalue_10) (.location _returnvalue_10) (.rotation _returnvalue_10))))
                              (Utilities|Array|SetArrayElem (Variables|/Game/BluePrints/Player/BP_InventoryComponent.BP_InventoryComponent_C|GetItems _bp_inventorycomponent) (Variables|/Game/BluePrints/Player/BP_InventoryComponent.BP_InventoryComponent_C|GetCurrentSlotIndex _bp_inventorycomponent) _output_get_5)
                              (Default|ResizeandLoad _bp_inventorycomponent)
                              (Actor|DestroyActor (Variables|/Game/BluePrints/Player/BP_InventoryComponent.BP_InventoryComponent_C|GetHoldItem _bp_inventorycomponent))
                              (Development|PrintString "холодная вода"))))))
                    (:NewEnumerator17
                      (bind _returnvalue_11 (Utilities|GetDataTableRow "/Game/BluePrints/Resources/DT_ItemsInventor.DT_ItemsInventor" "Bucket_ColdWater1")
                        (:then
                          (Default|ApplyItemData _asbp_item _returnvalue_11)
                          (goto _label))))
                    (:NewEnumerator18
                      (bind _returnvalue_12 (Utilities|GetDataTableRow "/Game/BluePrints/Resources/DT_ItemsInventor.DT_ItemsInventor" "Bucket_ColdWater2")
                        (:then
                          (Default|ApplyItemData _asbp_item _returnvalue_12)
                          (goto _label))))
                    (:NewEnumerator9
                      (bind _returnvalue_13 (Utilities|GetDataTableRow "/Game/BluePrints/Resources/DT_ItemsInventor.DT_ItemsInventor" "Bucket_Empty")
                        (:then
                          (Default|ApplyItemData _asbp_item _returnvalue_13)
                          (bind _returnvalue_14 (Utilities|GetDataTableRow "/Game/BluePrints/Resources/DT_ItemsInventor.DT_ItemsInventor" "Flask_Water" :!label _label_2)
                            (:then
                              (bind _output_get_6 (Variables|/Game/BluePrints/BP_Item.BP_Item_C|SetItem (Variables|/Game/BluePrints/Player/BP_InventoryComponent.BP_InventoryComponent_C|GetHoldItem (Variables|/Game/BluePrints/Player/BP_PlayerCharacter.BP_PlayerCharacter_C|GetBP_InventoryComponent (Variables|Default|GetPlayerCharacter))) (Utilities|Struct|MakeSTR_ItemsInventory (.name _returnvalue_14) (.icon _returnvalue_14) (.mesh _returnvalue_14) (.stackabled _returnvalue_14) (.quanity _returnvalue_14) (.maxstackebled _returnvalue_14) (.scale _returnvalue_14) (.enum _returnvalue_14) (.location _returnvalue_14) (.rotation _returnvalue_14))))
                              (Utilities|Array|SetArrayElem (Variables|/Game/BluePrints/Player/BP_InventoryComponent.BP_InventoryComponent_C|GetItems _bp_inventorycomponent_3) (Variables|/Game/BluePrints/Player/BP_InventoryComponent.BP_InventoryComponent_C|GetCurrentSlotIndex _bp_inventorycomponent_3) _output_get_6)
                              (Default|ResizeandLoad _bp_inventorycomponent_3)
                              (Actor|DestroyActor (Variables|/Game/BluePrints/Player/BP_InventoryComponent.BP_InventoryComponent_C|GetHoldItem _bp_inventorycomponent_3)))))))
                    (:NewEnumerator14
                      (bind _returnvalue_15 (Utilities|GetDataTableRow "/Game/BluePrints/Resources/DT_ItemsInventor.DT_ItemsInventor" "Bucket_Water1")
                        (:then
                          (Default|ApplyItemData _asbp_item _returnvalue_15)
                          (goto _label_2))))
                    (:NewEnumerator15
                      (bind _returnvalue_16 (Utilities|GetDataTableRow "/Game/BluePrints/Resources/DT_ItemsInventor.DT_ItemsInventor" "Bucket_Water2")
                        (:then
                          (Default|ApplyItemData _asbp_item _returnvalue_16)
                          (goto _label_2)))))))))))))
  (:Released
    (Variables|Default|SetisHoldingKey false)
    (Variables|/Game/BluePrints/Player/BP_PlayerCharacter.BP_PlayerCharacter_C|SetIsFishing (Variables|Default|GetPlayerCharacter) false)))

(event Input|ActionEvents|InputActionBuild
  (params (Key :type Key%20Structure :default "None"))
  (bind (_start _end) (Utilities|TraceLocations))
  (bind _holdbuild (Variables|Default|GetHoldBuild))
  (bind _playercharacter (Variables|Default|GetPlayerCharacter))
  (bind _bp_inventorycomponent (Variables|/Game/BluePrints/Player/BP_PlayerCharacter.BP_PlayerCharacter_C|GetBP_InventoryComponent _playercharacter))
  (bind _holditem (Variables|/Game/BluePrints/Player/BP_InventoryComponent.BP_InventoryComponent_C|GetHoldItem _bp_inventorycomponent))
  ;[0.15 0.15 0.15 0.5] Build
  (:Pressed
    (Variables|Default|SetisHoldingKey true)
    (if (Variables|Default|GetisChangeLocation)
      (if (Variables|Default|GetisCanBuild)
        (Variables|Default|SetisChangeLocation false)
        (Utilities|IsValid _holdbuild
          (:Is%20Valid
            (Default|SetSelfMaterial _holdbuild)
            (Variables|/Game/BluePrints/Building/BP_Build.BP_Build_C|SetisBuilt _holdbuild true)
            (bind _asbp_tent (Utilities|Casting|CastToBP_Tent (Variables|Default|GetHoldBuild)))
            (Default|SpawnResident _asbp_tent))))
      (elif (not (Variables|/Game/BluePrints/Player/BP_InventoryComponent.BP_InventoryComponent_C|GetisFreeHand (Variables|/Game/BluePrints/Player/BP_PlayerCharacter.BP_PlayerCharacter_C|GetBP_InventoryComponent (Variables|Default|GetPlayerCharacter))))
        (Utilities|IsValid _holditem
          (:Is%20Valid
            (switch Utilities|FlowControl|Switch|SwitchonENUM_Item (.Enum (Utilities|Struct|BreakSTR_ItemsInventory (Variables|/Game/BluePrints/BP_Item.BP_Item_C|GetItem _holditem)))
              (:NewEnumerator0
                (bind _outhit (Collision|LineTraceByChannel _start _end "TraceTypeQuery1" false 0 "None"))
                (Utilities|Casting|CastToLandscape (.HitActor (Collision|BreakHitResult _outhit)))
                (bind _returnvalue (UserInterface|CreateWidget "/Game/WidgetBlueprints/WBP_Building.WBP_Building_C"))
                (bind _output_get (Variables|Default|SetWBP_Building _returnvalue))
                (UserInterface|Viewport|AddtoViewport _output_get 0)
                (Variables|/Game/BluePrints/Player/BP_PlayerCharacter.BP_PlayerCharacter_C|SetisRotateCamera (Variables|Default|GetPlayerCharacter) false)
                (Variables|/Script/Engine.PlayerController|SetbShowMouseCursor (Variables|Default|GetPlayerController) true))))))))
  (:Released
    (Variables|Default|SetisHoldingKey false)))

(event Input|ActionEvents|InputActionSleep
  (params (Key :type Key%20Structure :default "None"))
  (bind (_start _end) (Utilities|TraceLocations))
  (bind _gamemode (Variables|Default|GetGameMode))
  (bind _sunmoon (Variables|/Game/BluePrints/BP_GameMode.BP_GameMode_C|GetSunMoon _gamemode))
  (bind _returnvalue (Class|DaySequenceActor|GetTimeOfDay _sunmoon))
  (bind _returnvalue_2 (Math|Float|Floor _returnvalue))
  ;[0.15 0.15 0.15 0.5] Sleep
  (:Pressed
    (bind _outhit (Collision|LineTraceByChannel _start _end "TraceTypeQuery1" false 0 "None"))
    (bind _asbp_player_tent (Utilities|Casting|CastToBP_PlayerTent (.HitActor (Collision|BreakHitResult _outhit))))
    (Utilities|IsValid (Variables|/Game/BluePrints/Building/BP_PlayerTent.BP_PlayerTent_C|Get%20BP%20Fire _asbp_player_tent)
      (:Is%20Valid
        (if (Variables|/Game/BluePrints/Building/BP_PlayerTent.BP_PlayerTent_C|GetisCanSleep _asbp_player_tent)
          (if (Variables|/Game/BluePrints/Player/BP_PlayerCharacter.BP_PlayerCharacter_C|GetisCanSleep (Variables|Default|GetPlayerCharacter))
            (if (and (> _returnvalue_2 6) (< _returnvalue_2 18))
              (CallFunction|Hint "Дождитесь ночи чтобы поспать" true)
              (else
                (Class|DaySequenceActor|SetTimeOfDay (Variables|/Game/BluePrints/BP_GameMode.BP_GameMode_C|GetSunMoon (Variables|Default|GetGameMode)) 8.0)
                (Default|Sleep _asbp_player_tent)
                (Default|Sleep (Variables|Default|GetPlayerCharacter))))
            (else
              (CallFunction|Hint "Лягьте на кровать" true)))
          (else
            (CallFunction|Hint "Тепла костра не хватит на всю ночь" true))))
      (:Is%20Not%20Valid
        (CallFunction|Hint "Необходим костер рядом для сна" true)))))

(event Input|KeyboardEvents|R
  (params (Key :type Key%20Structure :default "None"))
  (bind _playercharacter (Variables|Default|GetPlayerCharacter))
  (bind _playercharacter_2 (Variables|Default|GetPlayerCharacter))
  (bind _playercharacter_3 (Variables|Default|GetPlayerCharacter))
  (bind _playercharacter_4 (Variables|Default|GetPlayerCharacter))
  (bind _bp_sliderscomponent (Variables|/Game/BluePrints/Player/BP_PlayerCharacter.BP_PlayerCharacter_C|GetBP_SlidersComponent _playercharacter))
  (bind _bp_inventorycomponent (Variables|/Game/BluePrints/Player/BP_PlayerCharacter.BP_PlayerCharacter_C|GetBP_InventoryComponent _playercharacter_3))
  (bind _bp_inventorycomponent_2 (Variables|/Game/BluePrints/Player/BP_PlayerCharacter.BP_PlayerCharacter_C|GetBP_InventoryComponent _playercharacter_4))
  (bind _holditem (Variables|/Game/BluePrints/Player/BP_InventoryComponent.BP_InventoryComponent_C|GetHoldItem _bp_inventorycomponent))
  ;[0.15 0.15 0.15 0.5] Eat
  (:Pressed
    (Utilities|IsValid _holditem
      (:Is%20Valid
        (switch Utilities|FlowControl|Switch|SwitchonENUM_Item (.Enum (Utilities|Struct|BreakSTR_ItemsInventory (Variables|/Game/BluePrints/BP_Item.BP_Item_C|GetItem _holditem)))
          (:NewEnumerator5
            (Default|Eat (Variables|/Game/BluePrints/Player/BP_PlayerCharacter.BP_PlayerCharacter_C|GetBP_SlidersComponent _playercharacter_2) 25.0)
            (Actor|DestroyActor (Variables|/Game/BluePrints/Player/BP_InventoryComponent.BP_InventoryComponent_C|GetHoldItem (Variables|/Game/BluePrints/Player/BP_PlayerCharacter.BP_PlayerCharacter_C|GetBP_InventoryComponent _playercharacter_2)))
            (Default|RemoveItem _bp_inventorycomponent_2 (Variables|/Game/BluePrints/Player/BP_InventoryComponent.BP_InventoryComponent_C|GetCurrentSlotIndex _bp_inventorycomponent_2) 1)
            (Audio|PlaySound2D "/Game/Assets/Audio/Sounds/Eating.Eating" 1.0 1.0 0.0 0 0))
          (:NewEnumerator13
            (Default|Drink _bp_sliderscomponent 25.0 false)
            (Default|RemoveItem (Variables|/Game/BluePrints/Player/BP_PlayerCharacter.BP_PlayerCharacter_C|GetBP_InventoryComponent (Variables|Default|GetPlayerCharacter)) (Variables|/Game/BluePrints/Player/BP_InventoryComponent.BP_InventoryComponent_C|GetCurrentSlotIndex (Variables|/Game/BluePrints/Player/BP_PlayerCharacter.BP_PlayerCharacter_C|GetBP_InventoryComponent _playercharacter)) 1 :!label _label)
            (Actor|DestroyActor (Variables|/Game/BluePrints/Player/BP_InventoryComponent.BP_InventoryComponent_C|GetHoldItem (Variables|/Game/BluePrints/Player/BP_PlayerCharacter.BP_PlayerCharacter_C|GetBP_InventoryComponent (Variables|Default|GetPlayerCharacter))))
            (bind _returnvalue (Utilities|GetDataTableRow "/Game/BluePrints/Resources/DT_ItemsInventor.DT_ItemsInventor" "Flask_empty")
              (:then
                (Default|AddItem (Variables|/Game/BluePrints/Player/BP_PlayerCharacter.BP_PlayerCharacter_C|GetBP_InventoryComponent (Variables|Default|GetPlayerCharacter)) _returnvalue)
                (Audio|PlaySound2D "/Game/Assets/Audio/Sounds/Drink.Drink" 1.0 1.0 0.0 0 0)
                (bind _returnvalue_2 (Utilities|GetDataTableRow "/Game/BluePrints/Resources/DT_ItemsInventor.DT_ItemsInventor" "Flask_empty")
                  (:then
                    (Variables|/Game/BluePrints/BP_Item.BP_Item_C|SetItem (Variables|/Game/BluePrints/Player/BP_InventoryComponent.BP_InventoryComponent_C|GetHoldItem (Variables|/Game/BluePrints/Player/BP_PlayerCharacter.BP_PlayerCharacter_C|GetBP_InventoryComponent (Variables|Default|GetPlayerCharacter))) _returnvalue_2))))))
          (:NewEnumerator16
            (Default|Drink _bp_sliderscomponent 25.0 true)
            (goto _label)))))))

(event Input|MouseEvents|LeftMouseButton
  (params (Key :type Key%20Structure :default "None")))

(fn TryInteract)

(fn SetCurrentInteractable
  (params (NewInteractable :type Actor%20Object%20Reference))
  (Variables|Default|SetCurrentInteractable NewInteractable))

(fn ClearCurrentInteractable
  (params (InteractableToClear :type Actor%20Object%20Reference))
  (if (== (Variables|Default|GetCurrentInteractable) InteractableToClear)
    (Variables|Default|SetCurrentInteractable 0)))