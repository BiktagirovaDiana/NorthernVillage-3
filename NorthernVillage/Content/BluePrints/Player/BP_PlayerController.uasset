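; Player controller that handles pause input and mouse-wheel control of the hotbar and building placement.
; On begin play it caches the player character and its inventory and interaction components.
; The wheel yaws the held build while rotate mode is on; otherwise it steps the inventory slot index with wrap-around and calls GetItem.
; Pause pauses the game and creates the pause widget.
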(event EventBeginPlay
  (bind _asbp_player_character (Utilities|Casting|CastToBP_PlayerCharacter (Game|Player|GetPlayerPawn 0)))
  (bind _output_get (Variables|Default|SetBP%20Player%20Character _asbp_player_character))
  (Variables|Default|SetBP%20Inventory%20Component (Variables|/Game/BluePrints/Player/BP_PlayerCharacter.BP_PlayerCharacter_C|GetBP_InventoryComponent _output_get))
  (Variables|Default|SetBP%20Interaction%20Component (Variables|/Game/BluePrints/Player/BP_PlayerCharacter.BP_PlayerCharacter_C|GetBP_InteractionComponent _output_get)))

(event EventTick
  (params (DeltaSeconds :type Float%20%28single-precision%29)))

(event Input|ActionEvents|InputActionPause
  (params (Key :type Key%20Structure :default "None"))
  (:Pressed
    (Game|SetGamePaused true)
    (UserInterface|CreateWidget "/Game/WidgetBlueprints/WBP_Pause.WBP_Pause_C")))

(event Input|AxisEvents|InputAxisMouseWheel
  (params (AxisValue :type Float%20%28single-precision%29))
  (bind _bp_inventory_component (Variables|Default|GetBP%20Inventory%20Component))
  (if (Variables|/Game/BluePrints/Player/BP_InteractionComponent.BP_InteractionComponent_C|GetisRotateBuild (Variables|Default|GetBP%20Interaction%20Component))
    (Transformation|SetActorRotation (Variables|/Game/BluePrints/Player/BP_InteractionComponent.BP_InteractionComponent_C|GetHoldBuild (Variables|Default|GetBP%20Interaction%20Component)) (Math|Rotator|MakeRotator 0.0 0.0 (+ (* AxisValue 1e+01) (+ 0.0 (.Yaw (Math|Rotator|BreakRotator (Transformation|GetActorRotation (Variables|/Game/BluePrints/Player/BP_InteractionComponent.BP_InteractionComponent_C|GetHoldBuild (Variables|Default|GetBP%20Interaction%20Component)))))))))
    (elif (!= AxisValue 0.0)
      (if (> (+ (Variables|/Game/BluePrints/Player/BP_InventoryComponent.BP_InventoryComponent_C|GetCurrentSlotIndex (Variables|Default|GetBP%20Inventory%20Component)) (Math|Float|Round AxisValue)) 8)
        (Variables|/Game/BluePrints/Player/BP_InventoryComponent.BP_InventoryComponent_C|SetCurrentSlotIndex _bp_inventory_component 0)
        (elif (< (+ (Variables|/Game/BluePrints/Player/BP_InventoryComponent.BP_InventoryComponent_C|GetCurrentSlotIndex (Variables|Default|GetBP%20Inventory%20Component)) (Math|Float|Round AxisValue)) 0)
          (Variables|/Game/BluePrints/Player/BP_InventoryComponent.BP_InventoryComponent_C|SetCurrentSlotIndex _bp_inventory_component 8)
          (else
            (Variables|/Game/BluePrints/Player/BP_InventoryComponent.BP_InventoryComponent_C|SetCurrentSlotIndex (Variables|Default|GetBP%20Inventory%20Component) (+ (Variables|/Game/BluePrints/Player/BP_InventoryComponent.BP_InventoryComponent_C|GetCurrentSlotIndex (Variables|Default|GetBP%20Inventory%20Component)) (Math|Float|Round AxisValue))))))
      (Default|GetItem _bp_inventory_component))))

(fn ConstructionScript)