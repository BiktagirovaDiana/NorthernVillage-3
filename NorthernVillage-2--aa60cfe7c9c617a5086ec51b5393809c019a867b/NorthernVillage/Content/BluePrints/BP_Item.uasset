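; BP_Item is a world item whose behavior switches on its item type, with data set directly or loaded by row from DT_ItemsInventor.
; Torches light up, burn down on a looping timer until destroyed, and toggle the player's cold state through WarmBox overlaps.
; In fire, raw fish swaps to the fried fish row after a timer, and water buckets can emit steam.
; Dropping resets rotation and heavily damps some bucket types.
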(event OnComponentBeginOverlap(WarmBox)
  (params (OverlappedComponent :type Primitive%20Component%20Object%20Reference) (OtherActor :type Actor%20Object%20Reference) (OtherComp :type Primitive%20Component%20Object%20Reference) (OtherBodyIndex :type Integer) (bFromSweep :type Boolean) (SweepResult :type Hit%20Result%20Structure%20%28by%20ref%29))
  (switch Utilities|FlowControl|Switch|SwitchonENUM_Item (.Enum (Utilities|Struct|BreakSTR_ItemsInventory (Variables|Default|GetItem)))
    (:NewEnumerator11
      (bind _returnvalue (Utilities|Time|SetTimerbyEvent (delegate Custom|CheckIsWarm) (Utilities|Time|GetWorldDeltaSeconds) true))
      (Variables|Default|SetTimertWarm _returnvalue))))

(event OnComponentEndOverlap(WarmBox)
  (params (OverlappedComponent :type Primitive%20Component%20Object%20Reference) (OtherActor :type Actor%20Object%20Reference) (OtherComp :type Primitive%20Component%20Object%20Reference) (OtherBodyIndex :type Integer))
  (switch Utilities|FlowControl|Switch|SwitchonENUM_Item (.Enum (Utilities|Struct|BreakSTR_ItemsInventory (Variables|Default|GetItem)))
    (:NewEnumerator11
      (Variables|/Game/BluePrints/Player/BP_SlidersComponent.BP_SlidersComponent_C|SetisCold (Variables|/Game/BluePrints/Player/BP_PlayerCharacter.BP_PlayerCharacter_C|GetBP_SlidersComponent (Variables|Default|GetPlayer%20Character)) true))))

(event Custom|CheckIsWarm
  (Variables|/Game/BluePrints/Player/BP_SlidersComponent.BP_SlidersComponent_C|SetisCold (Variables|/Game/BluePrints/Player/BP_PlayerCharacter.BP_PlayerCharacter_C|GetBP_SlidersComponent (Variables|Default|GetPlayer%20Character)) false)
  (Utilities|Time|ClearandInvalidateTimerbyHandle (Variables|Default|GetTimertWarm)))

(event Custom|StartCookInFire
  (Variables|Default|SetbIsInFire true)
  (if (== (Variables|Default|GetItemRowName) "Fish_Raw")
    (Utilities|Time|ClearandInvalidateTimerbyHandle (Variables|Default|GetCookTimerHandle))
    (bind _returnvalue (Utilities|Time|SetTimerbyEvent (delegate Custom|FinishCooking) 5.0))
    (Variables|Default|SetCookTimerHandle _returnvalue)))

(event Custom|FinishCooking
  (if (Variables|Default|GetbIsInFire)
    (if (== (Variables|Default|GetItemRowName) "Fish_Raw")
      (bind _returnvalue (Utilities|GetDataTableRow "/Game/BluePrints/Resources/DT_ItemsInventor.DT_ItemsInventor" "Fried_Fish")
        (:then
          (Variables|Default|SetItemRowName "Fried_Fish")
          (CallFunction|ApplyItemData (Utilities|Struct|MakeSTR_ItemsInventory (.name _returnvalue) (.icon _returnvalue) (.mesh _returnvalue) (.stackabled _returnvalue) (.quanity _returnvalue) (.maxstackebled _returnvalue) (.scale _returnvalue) (.enum _returnvalue) (.location _returnvalue) (.rotation _returnvalue))))))))

(event Custom|StopSteamInFire
  (Variables|Default|SetbIsInFire false)
  (Utilities|Time|ClearandInvalidateTimerbyHandle (Variables|Default|GetSteamTimerHandle))
  (Components|Activation|Deactivate (Variables|Default|GetSteamFX)))

(event Custom|UpdateMesh
  (bind _mesh (Variables|Default|GetMesh))
  (bind _item (Variables|Default|GetItem))
  (bind (_name _icon _mesh_2 _stackabled _quanity _maxstackebled _scale) (Utilities|Struct|BreakSTR_ItemsInventory _item))
  (Components|StaticMesh|SetStaticMesh _mesh _mesh_2)
  (Transformation|SetWorldScale3D _mesh _scale))

(event Custom|Drop
  (Transformation|SetWorldRotation (Variables|Default|GetMesh) "0, 0, 0" false false)
  (Transformation|SetRelativeRotation (Variables|Default|GetMesh) "0, 0, 0" false false)
  (Transformation|SetActorRelativeRotation "0, 0, 0")
  (switch Utilities|FlowControl|Switch|SwitchonENUM_Item (.Enum (Utilities|Struct|BreakSTR_ItemsInventory (Variables|Default|GetItem)))
    (:NewEnumerator1
      _)
    (:NewEnumerator7
      _)
    (:NewEnumerator6
      _))
  (Class|PrimitiveComponent|SetAngularDamping (Variables|Default|GetMesh) 5e+01))

(event Custom|Burn
  (if (< (Variables|Default|GetTime) (Variables|Default|GetTimer))
    (Variables|Default|SetTime (+ (Variables|Default|GetTime) 1.0))
    (else
      (Actor|DestroyActor))))

(event Custom|StartSteam
  (bind _steamfx (Variables|Default|GetSteamFX))
  (switch Utilities|FlowControl|Switch|SwitchonENUM_Item (.Enum (Utilities|Struct|BreakSTR_ItemsInventory (Variables|Default|GetItem)))
    (:NewEnumerator9
      (Components|Activation|Activate _steamfx false)
      (Components|Activation|SetActive _steamfx true false))))

(event EventBeginPlay
  (bind _asbp_player_character (Utilities|Casting|CastToBP_PlayerCharacter (Game|Player|GetPlayerPawn 0)))
  (Variables|Default|SetPlayer%20Character _asbp_player_character)
  (Transformation|SetWorldScale3D (Variables|Default|GetMesh) (.Scale (Utilities|Struct|BreakSTR_ItemsInventory (Variables|Default|GetItem))))
  (Rendering|SetVisibility (Variables|Default|GetPointLight) false false)
  (Rendering|SetVisibility (Variables|Default|GetParticleSystem) false false)
  (switch Utilities|FlowControl|Switch|SwitchonENUM_Item (.Enum (Utilities|Struct|BreakSTR_ItemsInventory (Variables|Default|GetItem)))
    (:NewEnumerator11
      (Variables|Default|SetTime 0.0)
      (Variables|Default|SetTimer 5e+01)
      (Rendering|SetVisibility (Variables|Default|GetParticleSystem) true false)
      (Rendering|SetVisibility (Variables|Default|GetPointLight) true false)
      (Utilities|Time|SetTimerbyEvent (delegate Custom|Burn) 0.5 true))))

(event Collision|EventActorBeginOverlap
  (params (OtherActor :type Actor%20Object%20Reference)))

(event EventTick
  (params (DeltaSeconds :type Float%20%28single-precision%29)))

(fn ConstructionScript
  (bind _mesh (Variables|Default|GetMesh))
  (Components|StaticMesh|SetStaticMesh _mesh (.Mesh (Utilities|Struct|BreakSTR_ItemsInventory (Variables|Default|GetItem))))
  (Transformation|SetWorldScale3D _mesh "0.002000,0.002000,0.002000"))

(fn ApplyItemData
  (params (NewItem :type STR%20Items%20Inventory%20Structure))
  (Variables|Default|SetItem NewItem)
  (Components|StaticMesh|SetStaticMesh (Variables|Default|GetMesh) (.Mesh (Utilities|Struct|BreakSTR_ItemsInventory NewItem))))

(fn StopCookinFire
  (Variables|Default|SetbIsInFire false)
  (Utilities|Time|ClearandInvalidateTimerbyHandle (Variables|Default|GetCookTimerHandle)))

(fn InitfromRowName
  (params (RowName :type Name))
  (Variables|Default|SetItemRowName RowName)
  (bind _returnvalue (Utilities|GetDataTableRow "/Game/BluePrints/Resources/DT_ItemsInventor.DT_ItemsInventor" RowName)
    (:then
      (Variables|Default|SetItem _returnvalue)
      (CallFunction|UpdateMesh))))