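; Player inventory component that manages a nine-slot hotbar, the item in the player's hand, and pickup and drop.
; StartGame creates WBP_Inventory and seeds starter tools from DT_ItemsInventor; inventory changes reload the widget.
; Pickup line-traces for BP_Item actors and stacks them, while number keys spawn the slot's item as a physics-disabled actor on HoldPoint.
; Q detaches it with physics and decrements the slot, respawning one in hand while stock remains.
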(event Custom|GetItem
  (bind _items (Variables|Default|GetItems))
  (bind _ischangeitem (Variables|Default|GetisChangeItem))
  (bind _currentslotindex (Variables|Default|GetCurrentSlotIndex))
  (bind _playercharacter (Variables|Default|GetPlayerCharacter))
  (bind _output (Utilities|Array|Get(acopy) _items _currentslotindex))
  (bind (_name _icon _mesh _stackabled _quanity _maxstackebled _scale _enum _location _rotation) (Utilities|Struct|BreakSTR_ItemsInventory _output))
  ;[0.15 0.15 0.15 0.5] Get item
  (if (Utilities|Array|Get(acopy) (Variables|Default|GetisChangeItem) (Variables|Default|GetCurrentSlotIndex))
    (Utilities|Array|SetArrayElem (Variables|Default|GetisChangeItem) (Variables|Default|GetCurrentSlotIndex) false)
    (Utilities|IsValid (Variables|Default|GetHoldItem)
      (:Is%20Valid
        (Actor|DestroyActor (Variables|Default|GetHoldItem))
        (Variables|Default|SetHoldItem 0)
        (Variables|Default|SetisFreeHand false))
      (:Is%20Not%20Valid
        (Variables|Default|SetisFreeHand false)))
    (else
      (for (_ _array_index) _ischangeitem
        (Utilities|Array|SetArrayElem _ischangeitem _array_index false))
      (Utilities|Array|SetArrayElem _ischangeitem (Variables|Default|GetCurrentSlotIndex) true)
      (CallFunction|ResizeandLoad)
      (Utilities|IsValid (Variables|Default|GetHoldItem)
        (:Is%20Valid
          (Actor|DestroyActor (Variables|Default|GetHoldItem)))
        (:Is%20Not%20Valid
          _))
      (Variables|Default|SetisFreeHand false)
      (bind _returnvalue (Game|SpawnActorfromClass "/Game/BluePrints/BP_Item.BP_Item_C" (Math|Conversions|ToTransform(Vector) (Transformation|GetWorldLocation (Variables|/Game/BluePrints/Player/BP_PlayerCharacter.BP_PlayerCharacter_C|GetHoldPoint (Variables|Default|GetPlayerCharacter)))) "Undefined" "MultiplyWithRoot" 0 (Utilities|Struct|MakeSTR_ItemsInventory _name _icon _mesh _stackabled 1 _maxstackebled _scale _enum _location _rotation) (Utilities|String|StringToName (Utilities|String|ToString(Text) _name)) 0))
      (bind _output_get (Variables|Default|SetHoldItem _returnvalue))
      (Development|PrintString (Utilities|String|ToString(Vector) (.Location (Utilities|Struct|BreakSTR_ItemsInventory (Variables|/Game/BluePrints/BP_Item.BP_Item_C|GetItem _output_get)))))
      (Transformation|SetRelativeLocationAndRotation (Variables|/Game/BluePrints/Player/BP_PlayerCharacter.BP_PlayerCharacter_C|GetHoldPoint (Variables|Default|GetPlayerCharacter)) (.Location (Utilities|Struct|BreakSTR_ItemsInventory (Variables|/Game/BluePrints/BP_Item.BP_Item_C|GetItem _output_get))) (.Rotation (Utilities|Struct|BreakSTR_ItemsInventory (Variables|/Game/BluePrints/BP_Item.BP_Item_C|GetItem _output_get))) false false)
      (Physics|SetSimulatePhysics (Variables|/Game/BluePrints/BP_Item.BP_Item_C|GetMesh _returnvalue) false)
      (Collision|SetCollisionEnabled (Variables|/Game/BluePrints/BP_Item.BP_Item_C|GetMesh _returnvalue) "NoCollision")
      (Actor|SetOwner (Variables|Default|GetHoldItem) _playercharacter)
      (Transformation|AttachComponentToComponent (Variables|Default|GetHoldItem) (Variables|/Game/BluePrints/Player/BP_PlayerCharacter.BP_PlayerCharacter_C|GetHoldPoint _playercharacter) "None" "SnapToTarget" "SnapToTarget" "KeepWorld" true))))

(event Custom|RemoveItem
  (params (SlotIndex :type Integer) (NumberDropItems :type Integer))
  (bind _playercharacter (Variables|Default|GetPlayerCharacter))
  (Variables|Default|SetSlotIndex SlotIndex)
  (if (.Stackabled (Utilities|Struct|BreakSTR_ItemsInventory (Utilities|Array|Get(acopy) (Variables|Default|GetItems) (Variables|Default|GetSlotIndex))))
    (if (!= (.Quanity (Utilities|Struct|BreakSTR_ItemsInventory (Utilities|Array|Get(acopy) (Variables|Default|GetItems) (Variables|Default|GetSlotIndex)))) NumberDropItems)
      (Utilities|Array|SetArrayElem (Variables|Default|GetItems) (Variables|Default|GetSlotIndex) (Utilities|Struct|MakeSTR_ItemsInventory (.Name (Utilities|Struct|BreakSTR_ItemsInventory (Utilities|Array|Get(acopy) (Variables|Default|GetItems) (Variables|Default|GetSlotIndex)))) (.Icon (Utilities|Struct|BreakSTR_ItemsInventory (Utilities|Array|Get(acopy) (Variables|Default|GetItems) (Variables|Default|GetSlotIndex)))) (.Mesh (Utilities|Struct|BreakSTR_ItemsInventory (Utilities|Array|Get(acopy) (Variables|Default|GetItems) (Variables|Default|GetSlotIndex)))) (.Stackabled (Utilities|Struct|BreakSTR_ItemsInventory (Utilities|Array|Get(acopy) (Variables|Default|GetItems) (Variables|Default|GetSlotIndex)))) (- (.Quanity (Utilities|Struct|BreakSTR_ItemsInventory (Utilities|Array|Get(acopy) (Variables|Default|GetItems) (Variables|Default|GetSlotIndex)))) NumberDropItems) (.MaxStackebled (Utilities|Struct|BreakSTR_ItemsInventory (Utilities|Array|Get(acopy) (Variables|Default|GetItems) (Variables|Default|GetSlotIndex)))) (.Scale (Utilities|Struct|BreakSTR_ItemsInventory (Utilities|Array|Get(acopy) (Variables|Default|GetItems) (Variables|Default|GetSlotIndex)))) (.Enum (Utilities|Struct|BreakSTR_ItemsInventory (Utilities|Array|Get(acopy) (Variables|Default|GetItems) (Variables|Default|GetSlotIndex)))) (.Location (Utilities|Struct|BreakSTR_ItemsInventory (Utilities|Array|Get(acopy) (Variables|Default|GetItems) (Variables|Default|GetSlotIndex)))) (.Rotation (Utilities|Struct|BreakSTR_ItemsInventory (Utilities|Array|Get(acopy) (Variables|Default|GetItems) (Variables|Default|GetSlotIndex))))))
      (if (Variables|Default|GetisDrop)
        (bind _returnvalue (Game|SpawnActorfromClass "/Game/BluePrints/BP_Item.BP_Item_C" (Math|Conversions|ToTransform(Vector) (Transformation|GetWorldLocation (Variables|/Game/BluePrints/Player/BP_PlayerCharacter.BP_PlayerCharacter_C|GetHoldPoint (Variables|Default|GetPlayerCharacter)))) "Undefined" "MultiplyWithRoot" 0 (Utilities|Struct|MakeSTR_ItemsInventory (.Name (Utilities|Struct|BreakSTR_ItemsInventory (Utilities|Array|Get(acopy) (Variables|Default|GetItems) (Variables|Default|GetSlotIndex)))) (.Icon (Utilities|Struct|BreakSTR_ItemsInventory (Utilities|Array|Get(acopy) (Variables|Default|GetItems) (Variables|Default|GetSlotIndex)))) (.Mesh (Utilities|Struct|BreakSTR_ItemsInventory (Utilities|Array|Get(acopy) (Variables|Default|GetItems) (Variables|Default|GetSlotIndex)))) (.Stackabled (Utilities|Struct|BreakSTR_ItemsInventory (Utilities|Array|Get(acopy) (Variables|Default|GetItems) (Variables|Default|GetSlotIndex)))) NumberDropItems (.MaxStackebled (Utilities|Struct|BreakSTR_ItemsInventory (Utilities|Array|Get(acopy) (Variables|Default|GetItems) (Variables|Default|GetSlotIndex)))) (.Scale (Utilities|Struct|BreakSTR_ItemsInventory (Utilities|Array|Get(acopy) (Variables|Default|GetItems) (Variables|Default|GetSlotIndex)))) (.Enum (Utilities|Struct|BreakSTR_ItemsInventory (Utilities|Array|Get(acopy) (Variables|Default|GetItems) (Variables|Default|GetSlotIndex)))) (.Location (Utilities|Struct|BreakSTR_ItemsInventory (Utilities|Array|Get(acopy) (Variables|Default|GetItems) (Variables|Default|GetSlotIndex)))) (.Rotation (Utilities|Struct|BreakSTR_ItemsInventory (Utilities|Array|Get(acopy) (Variables|Default|GetItems) (Variables|Default|GetSlotIndex))))) "None" 0))
        (Variables|Default|SetHoldItem _returnvalue)
        (Physics|SetSimulatePhysics (Variables|/Game/BluePrints/BP_Item.BP_Item_C|GetMesh _returnvalue) false)
        (Collision|SetCollisionEnabled (Variables|/Game/BluePrints/BP_Item.BP_Item_C|GetMesh _returnvalue) "NoCollision")
        (Actor|SetOwner (Variables|Default|GetHoldItem) _playercharacter)
        (Transformation|AttachComponentToComponent (Variables|Default|GetHoldItem) (Variables|/Game/BluePrints/Player/BP_PlayerCharacter.BP_PlayerCharacter_C|GetHoldPoint _playercharacter) "None" "SnapToTarget" "SnapToTarget" "KeepWorld" true)
        (CallFunction|ResizeandLoad)
        (else
          (CallFunction|ResizeandLoad)))
      (else
        (Utilities|Array|RemoveIndex (Variables|Default|GetItems) (Variables|Default|GetSlotIndex) :!label _label)
        (Utilities|Array|SetArrayElem (Variables|Default|GetisChangeItem) (Variables|Default|GetSlotIndex) false)
        (CallFunction|ResizeandLoad)))
    (else
      (goto _label))))

(event Custom|Timer
  ;[0.15 0.15 0.15 0.5] Drop
  (Variables|Default|SetCanUsePressed true))

(event Custom|AddItem
  (params (STR_ITEM :type STR%20Items%20Inventory%20Structure))
  (bind (_name _icon _mesh _stackabled _quanity _maxstackebled _scale _enum _location _rotation) (Utilities|Struct|BreakSTR_ItemsInventory STR_ITEM))
  (bind (_name_2 _icon_2 _mesh_2 _stackabled_2 _quanity_2 _maxstackebled_2) (Utilities|Struct|BreakSTR_ItemsInventory STR_ITEM))
  ;[0.15 0.15 0.15 0.5] Add item in inventory
  (Variables|Default|SetIsEmpty true)
  (for (_array_element _array_index) (Variables|Default|GetItems)
    (if (Variables|Default|GetIsEmpty)
      (if (Math|Boolean|ANDBoolean (Utilities|Enum|Equal(Enum) (.Name (Utilities|Struct|BreakSTR_ItemsInventory _array_element)) _name_2) _stackabled_2 (<= (+ (.Quanity (Utilities|Struct|BreakSTR_ItemsInventory _array_element)) _quanity_2) _maxstackebled_2))
        (Utilities|Array|SetArrayElem (Variables|Default|GetItems) _array_index (Utilities|Struct|MakeSTR_ItemsInventory _name _icon _mesh _stackabled (+ (.Quanity (Utilities|Struct|BreakSTR_ItemsInventory _array_element)) _quanity_2) _maxstackebled _scale _enum _location _rotation))
        (Default|LoadInventory (Variables|Default|GetInventory) self :!label _label)
        (Variables|Default|SetIsEmpty false)
        (elif (== (.Quanity (Utilities|Struct|BreakSTR_ItemsInventory _array_element)) 0)
          (Utilities|Array|SetArrayElem (Variables|Default|GetItems) _array_index STR_ITEM)
          (goto _label))))))

(event Custom|StartGame
  (bind _returnvalue (UserInterface|CreateWidget "/Game/WidgetBlueprints/Inventory/WBP_Inventory.WBP_Inventory_C"))
  (bind _output_get (Variables|Default|SetInventory _returnvalue))
  (UserInterface|Viewport|AddtoViewport _output_get 0)
  (Utilities|Array|Resize (Variables|Default|GetItems) 9)
  (Default|LoadInventory (Variables|Default|GetInventory) self)
  (bind _asbp_player_character (Utilities|Casting|CastToBP_PlayerCharacter (Game|Player|GetPlayerPawn 0)))
  (Variables|Default|SetPlayerCharacter _asbp_player_character)
  (Variables|Default|SetMaxGragDistance 3e+02)
  (Variables|Default|SetisFreeHand true)
  (Utilities|Array|Resize (Variables|Default|GetisChangeItem) 8)
  (Variables|Default|SetCanUsePressed true)
  (Variables|Default|SetisDrop false)
  (bind _returnvalue_2 (Utilities|GetDataTableRow "/Game/BluePrints/Resources/DT_ItemsInventor.DT_ItemsInventor" "Bucket_Empty")
    (:then
      (CallFunction|AddItem _returnvalue_2)
      (bind _returnvalue_3 (Utilities|GetDataTableRow "/Game/BluePrints/Resources/DT_ItemsInventor.DT_ItemsInventor" "FishingRod")
        (:then
          (CallFunction|AddItem _returnvalue_3)
          (bind _returnvalue_4 (Utilities|GetDataTableRow "/Game/BluePrints/Resources/DT_ItemsInventor.DT_ItemsInventor" "Hammer")
            (:then
              (CallFunction|AddItem _returnvalue_4)
              (bind _returnvalue_5 (Utilities|GetDataTableRow "/Game/BluePrints/Resources/DT_ItemsInventor.DT_ItemsInventor" "Axe")
                (:then
                  (CallFunction|AddItem _returnvalue_5))))))))))

(event EventBeginPlay)

(event Input|ActionEvents|InputActionPickUp
  (params (Key :type Key%20Structure :default "None"))
  (bind (_startlocation _endlocation) (Utilities|TraceLocations))
  ;[0.15 0.15 0.15 0.5] Pick up item
  (:Pressed
    (bind _outhit (Collision|LineTraceByChannel _startlocation _endlocation "TraceTypeQuery1" false 0 "None"))
    (bind _asbp_item (Utilities|Casting|CastToBP_Item (.HitActor (Collision|BreakHitResult _outhit))))
    (CallFunction|AddItem (Variables|/Game/BluePrints/BP_Item.BP_Item_C|GetItem _asbp_item))
    (Actor|DestroyActor _asbp_item)))

(event Input|KeyboardEvents|DebugKeyQ
  (params (Key :type Key%20Structure :default "None") (ActionValue :type Input%20Action%20Value%20Structure))
  ;[0.15 0.15 0.15 0.5] Drop
  (:Pressed
    (if (Variables|Default|GetCanUsePressed)
      (Variables|Default|SetCanUsePressed false)
      (Utilities|Time|SetTimerbyEvent (delegate Custom|Timer) 0.5)
      (Variables|Default|SetisFreeHand true)
      (Utilities|IsValid (Variables|Default|GetHoldItem)
        (:Is%20Valid
          (Physics|SetSimulatePhysics (Variables|/Game/BluePrints/BP_Item.BP_Item_C|GetMesh (Variables|Default|GetHoldItem)) true)
          (Collision|SetCollisionEnabled (Variables|/Game/BluePrints/BP_Item.BP_Item_C|GetMesh (Variables|Default|GetHoldItem)) "QueryAndPhysics")
          (Actor|SetOwner (Variables|Default|GetHoldItem) 0)
          (Transformation|DetachFromActor (Variables|Default|GetHoldItem) "KeepWorld" "KeepWorld" "KeepWorld")
          (Class|PrimitiveComponent|SetMassOverrideinKg (Variables|/Game/BluePrints/BP_Item.BP_Item_C|GetMesh (Variables|Default|GetHoldItem)) "None" 2e+01 true)
          (Default|Drop (Variables|Default|GetHoldItem))
          (Variables|Default|SetHoldItem 0)
          (Variables|Default|SetisDrop true)
          (CallFunction|RemoveItem (Variables|Default|GetCurrentSlotIndex) 1)
          (Variables|Default|SetisDrop false))))))

(event Input|KeyboardEvents|5
  (params (Key :type Key%20Structure :default "None"))
  (:Pressed
    (Variables|Default|SetCurrentSlotIndex 4)
    (CallFunction|GetItem)))

(event Input|KeyboardEvents|1
  (params (Key :type Key%20Structure :default "None"))
  (:Pressed
    (Variables|Default|SetCurrentSlotIndex 0)
    (CallFunction|GetItem)))

(event Input|KeyboardEvents|9
  (params (Key :type Key%20Structure :default "None"))
  (:Pressed
    (Variables|Default|SetCurrentSlotIndex 8)
    (CallFunction|GetItem)))

(event Input|KeyboardEvents|2
  (params (Key :type Key%20Structure :default "None"))
  (:Pressed
    (Variables|Default|SetCurrentSlotIndex 1)
    (CallFunction|GetItem)))

(event Input|KeyboardEvents|3
  (params (Key :type Key%20Structure :default "None"))
  (:Pressed
    (Variables|Default|SetCurrentSlotIndex 2)
    (CallFunction|GetItem)))

(event Input|KeyboardEvents|4
  (params (Key :type Key%20Structure :default "None"))
  (:Pressed
    (Variables|Default|SetCurrentSlotIndex 3)
    (CallFunction|GetItem)))

(event Input|KeyboardEvents|6
  (params (Key :type Key%20Structure :default "None"))
  (:Pressed
    (Variables|Default|SetCurrentSlotIndex 5)
    (CallFunction|GetItem)))

(event Input|KeyboardEvents|7
  (params (Key :type Key%20Structure :default "None"))
  (:Pressed
    (Variables|Default|SetCurrentSlotIndex 6)
    (CallFunction|GetItem)))

(event Input|KeyboardEvents|8
  (params (Key :type Key%20Structure :default "None"))
  (:Pressed
    (Variables|Default|SetCurrentSlotIndex 7)
    (CallFunction|GetItem)))

(fn ResizeandLoad
  (Utilities|Array|Resize (Variables|Default|GetItems) 9)
  (Default|LoadInventory (Variables|Default|GetInventory) self))

(fn GetItemDatabyID
  (params (ItemID :type Name))
  (bind _returnvalue (Utilities|GetDataTableRow "/Game/BluePrints/Resources/DT_ItemsInventor.DT_ItemsInventor" ItemID)
    (:then
      (return _returnvalue true))
    (:RowNotFound
      (return "" false))))

(fn SetCurrentSlotItem
  (params (NewItem :type STR%20Items%20Inventory%20Structure))
  (Utilities|Array|SetArrayElem (Variables|Default|GetItems) (Variables|Default|GetCurrentSlotIndex) NewItem)
  (CallFunction|ResizeandLoad))

(fn CheckWood
  (params (NumberWood :type Integer))
  (bind _returnvalue (Utilities|GetDataTableRow "/Game/BluePrints/Resources/DT_ItemsInventor.DT_ItemsInventor" "Wood")
    (:then
      (for (_array_element _array_index) (Variables|Default|GetItems)
        (if (Utilities|Enum|Equal(Enum) (.Name (Utilities|Struct|BreakSTR_ItemsInventory _array_element)) (.Name (Utilities|Struct|BreakSTR_ItemsInventory _returnvalue)))
          (if (>= (.Quanity (Utilities|Struct|BreakSTR_ItemsInventory _array_element)) NumberWood)
            (return true _array_index NumberWood)
            (else
              (return false 0 0))))))))