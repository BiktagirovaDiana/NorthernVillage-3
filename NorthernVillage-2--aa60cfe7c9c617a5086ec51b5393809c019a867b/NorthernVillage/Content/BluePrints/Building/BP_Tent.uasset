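; BP_Tent is a building actor that houses one villager and shows that resident's house card to a nearby player.
; SpawnResident picks a random DT_Residents row once and spawns a BP_NPC_VillagerBase at the spawn point, linked back to the tent.
; A box overlap tracks player range; Z then opens WBP_HouseCard, pausing the game with UI-only input.
; ResidentRowName re-rolls the random index, so it can differ from the stored data.
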(event OnComponentBeginOverlap(Box)
  (params (OverlappedComponent :type Primitive%20Component%20Object%20Reference) (OtherActor :type Actor%20Object%20Reference) (OtherComp :type Primitive%20Component%20Object%20Reference) (OtherBodyIndex :type Integer) (bFromSweep :type Boolean) (SweepResult :type Hit%20Result%20Structure%20%28by%20ref%29))
  (Utilities|Casting|CastToBP_PlayerCharacter OtherActor)
  (Variables|Default|SetbPlayerInRange true))

(event OnComponentEndOverlap(Box)
  (params (OverlappedComponent :type Primitive%20Component%20Object%20Reference) (OtherActor :type Actor%20Object%20Reference) (OtherComp :type Primitive%20Component%20Object%20Reference) (OtherBodyIndex :type Integer))
  (Utilities|Casting|CastToBP_PlayerCharacter OtherActor)
  (Variables|Default|SetbPlayerInRange false))

(event Custom|OnClosed_Event
  (Variables|Default|SetHouseCardRef 0))

(event EventBeginPlay
  (|CallParentFunction) ; This node is disabled and will not be called.\nDrag off pins to build functionality.
)

(event Collision|EventActorBeginOverlap
  (params (OtherActor :type Actor%20Object%20Reference))
  (|CallParentFunction OtherActor) ; This node is disabled and will not be called.\nDrag off pins to build functionality.
)

(event EventTick
  (params (DeltaSeconds :type Float%20%28single-precision%29))
  (|CallParentFunction DeltaSeconds) ; This node is disabled and will not be called.\nDrag off pins to build functionality.
)

(event Input|KeyboardEvents|Z
  (params (Key :type Key%20Structure :default "None"))
  (bind _returnvalue (Game|GetPlayerController 0))
  (:Pressed
    (Development|PrintString "нажала z")
    (if (Variables|Default|GetbPlayerInRange)
      (Utilities|IsValid (Variables|Default|GetHouseCardRef)
        (:Is%20Not%20Valid
          (bind _returnvalue_2 (UserInterface|CreateWidget "/Game/WidgetBlueprints/WBP_HouseCard.WBP_HouseCard_C" 0 (Variables|Default|GetResidentData) (Variables|Default|GetResidentRef)))
          (UserInterface|Viewport|AddtoViewport _returnvalue_2 0)
          (EventDispatchers|AssignOnClosed _returnvalue_2 (delegate Custom|OnClosed_Event))
          (Input|SetInputModeUIOnly _returnvalue _returnvalue_2 "DoNotLock" false)
          (Variables|/Script/Engine.PlayerController|SetbShowMouseCursor _returnvalue true)
          (Game|SetGamePaused true))))))

(fn ConstructionScript
  (|CallParentFunction))

(fn SpawnResident
  (if (not (Variables|Default|GetbResidentSpawned))
    (bind _outrownames (DataTable|GetDataTableRowNames "/Game/BluePrints/AI/DT_Residents.DT_Residents"))
    (bind _returnvalue (Utilities|GetDataTableRow "/Game/BluePrints/AI/DT_Residents.DT_Residents" (Utilities|Array|Get(acopy) _outrownames (Math|Random|RandomIntegerinRange 0 (- (Utilities|Array|Length _outrownames) 1))))
      (:then
        (Variables|Default|SetResidentRowName (Utilities|Array|Get(acopy) _outrownames (Math|Random|RandomIntegerinRange 0 (- (Utilities|Array|Length _outrownames) 1))))
        (bind _output_get (Variables|Default|SetResidentData _returnvalue))
        (bind _returnvalue_2 (Game|SpawnActorfromClass "/Game/BluePrints/AI/BP_NPC_VillagerBase.BP_NPC_VillagerBase_C" (Transformation|GetWorldTransform (Variables|Default|GetResidentSpawnPoint)) "Undefined" "MultiplyWithRoot" 0 _output_get "None" 0))
        (Variables|/Game/BluePrints/AI/BP_NPC_VillagerBase.BP_NPC_VillagerBase_C|SetHomeTent _returnvalue_2 self)
        (Variables|Default|SetResidentRef _returnvalue_2)
        (Variables|Default|SetbResidentSpawned true)))))

(fn GetResidentReturnLocation
  (return (Transformation|GetWorldLocation (Variables|Default|GetResidentSpawnPoint))))