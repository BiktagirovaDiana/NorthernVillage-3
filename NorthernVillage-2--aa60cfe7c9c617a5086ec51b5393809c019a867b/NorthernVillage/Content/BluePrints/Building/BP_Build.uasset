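; BP_Build is a buildable object that shows whether its current spot is valid during placement.
; Until IsBuilt is set, RangeBuild overlaps with other BP_Build actors toggle the player interaction component's IsCanBuild and swap both meshes between CanBuild and CantBuild materials.
; The construction script caches each mesh's original material, which SetSelfMaterial restores.
; Any single end overlap re-allows building, as overlaps are not counted.
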(event OnComponentBeginOverlap(RangeBuild)
  (params (OverlappedComponent :type Primitive%20Component%20Object%20Reference) (OtherActor :type Actor%20Object%20Reference) (OtherComp :type Primitive%20Component%20Object%20Reference) (OtherBodyIndex :type Integer) (bFromSweep :type Boolean) (SweepResult :type Hit%20Result%20Structure%20%28by%20ref%29))
  (bind _playercharacter (Variables|Default|GetPlayerCharacter))
  (Utilities|Casting|CastToBP_Build OtherActor)
  (if (not (Variables|Default|GetisBuilt))
    (Utilities|IsValid _playercharacter
      (:Is%20Valid
        (Variables|/Game/BluePrints/Player/BP_InteractionComponent.BP_InteractionComponent_C|SetisCanBuild (Variables|/Game/BluePrints/Player/BP_PlayerCharacter.BP_PlayerCharacter_C|GetBP_InteractionComponent _playercharacter) false)
        (Rendering|Material|SetMaterial (Variables|Default|GetMesh1) 0 "/Game/BluePrints/Building/CantBuild.CantBuild")))))

(event OnComponentEndOverlap(RangeBuild)
  (params (OverlappedComponent :type Primitive%20Component%20Object%20Reference) (OtherActor :type Actor%20Object%20Reference) (OtherComp :type Primitive%20Component%20Object%20Reference) (OtherBodyIndex :type Integer))
  (Utilities|Casting|CastToBP_Build OtherActor)
  (if (not (Variables|Default|GetisBuilt))
    (Variables|/Game/BluePrints/Player/BP_InteractionComponent.BP_InteractionComponent_C|SetisCanBuild (Variables|/Game/BluePrints/Player/BP_PlayerCharacter.BP_PlayerCharacter_C|GetBP_InteractionComponent (Variables|Default|GetPlayerCharacter)) true)
    (Rendering|Material|SetMaterial (Variables|Default|GetMesh1) 0 "/Game/BluePrints/Building/CanBuild.CanBuild")))

(event Custom|SetSelfMaterial
  (Rendering|Material|SetMaterial (Variables|Default|GetMesh1) 0 (Variables|Default|GetSelfMaterial1))
  (Rendering|Material|SetMaterial (Variables|Default|GetMesh2) 0 (Variables|Default|GetSelfMaterial2)))

(event Custom|CanBuild
  (Rendering|Material|SetMaterial (Variables|Default|GetMesh1) 0 "/Game/BluePrints/Building/CanBuild.CanBuild")
  (Rendering|Material|SetMaterial (Variables|Default|GetMesh2) 0 "/Game/BluePrints/Building/CanBuild.CanBuild"))

(event EventBeginPlay
  (Variables|Default|SetisBuilt false)
  (bind _asbp_player_character (Utilities|Casting|CastToBP_PlayerCharacter (Game|Player|GetPlayerPawn 0)))
  (Variables|Default|SetPlayerCharacter _asbp_player_character)
  (if (Variables|Default|GetisBuilt)
    (CallFunction|SetSelfMaterial)))

(event Collision|EventActorBeginOverlap
  (params (OtherActor :type Actor%20Object%20Reference)))

(event EventTick
  (params (DeltaSeconds :type Float%20%28single-precision%29)))

(fn ConstructionScript
  (Variables|Default|SetSelfMaterial1 (Rendering|Material|GetMaterial (Variables|Default|GetMesh1) 0))
  (Variables|Default|SetSelfMaterial2 (Rendering|Material|GetMaterial (Variables|Default|GetMesh2) 0)))