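; Player tent that spawns its own campfire with both meshes hidden and lets the player sleep.
; A looping one-second timer sets the tent's sleep flag from the fire's Time value, while bed overlap toggles a separate flag on the player.
; Sleep lowers the player camera with a timeline, then destroys the fire and reverses the timeline to raise the camera again.
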(event OnComponentBeginOverlap(BedCollision)
  (params (OverlappedComponent :type Primitive%20Component%20Object%20Reference) (OtherActor :type Actor%20Object%20Reference) (OtherComp :type Primitive%20Component%20Object%20Reference) (OtherBodyIndex :type Integer) (bFromSweep :type Boolean) (SweepResult :type Hit%20Result%20Structure%20%28by%20ref%29))
  (bind _asbp_player_character (Utilities|Casting|CastToBP_PlayerCharacter OtherActor))
  (Variables|/Game/BluePrints/Player/BP_PlayerCharacter.BP_PlayerCharacter_C|SetisCanSleep _asbp_player_character true))

(event OnComponentEndOverlap(BedCollision)
  (params (OverlappedComponent :type Primitive%20Component%20Object%20Reference) (OtherActor :type Actor%20Object%20Reference) (OtherComp :type Primitive%20Component%20Object%20Reference) (OtherBodyIndex :type Integer))
  (bind _asbp_player_character (Utilities|Casting|CastToBP_PlayerCharacter OtherActor))
  (Variables|/Game/BluePrints/Player/BP_PlayerCharacter.BP_PlayerCharacter_C|SetisCanSleep _asbp_player_character false))

(event Custom|CheckFireEvent
  (bind __bp_fire (Variables|Default|Get%20BP%20Fire))
  (Utilities|IsValid __bp_fire
    (:Is%20Valid
      (if (<= (Variables|/Game/BluePrints/Building/BP_Fire.BP_Fire_C|GetTime __bp_fire) 25.0)
        (Variables|Default|SetisCanSleep true)
        (else
          (Variables|Default|SetisCanSleep false))))))

(event Custom|Sleep
  (bind __bp_fire (Variables|Default|Get%20BP%20Fire))
  (bind _alpha (Timeline|AnimCamera Play)
    (:Update
      (Transformation|SetRelativeLocation (Variables|/Game/BluePrints/Player/BP_PlayerCharacter.BP_PlayerCharacter_C|GetCamera (Variables|Default|Get%20Player%20Character)) (Math|Vector|MakeVector 0.0 0.0 (Math|Float|Lerp 7e+01 -2e+01 _alpha)) false false))
    (:Finished
      (Utilities|IsValid __bp_fire
        (:Is%20Valid
          (Actor|DestroyActor __bp_fire)
          (Timeline|AnimCamera Reverse))))))

(event EventBeginPlay
  (|CallParentFunction)
  (Utilities|Time|SetTimerbyEvent (delegate Custom|CheckFireEvent) 1.0 true)
  (bind _asbp_player_character (Utilities|Casting|CastToBP_PlayerCharacter (Game|Player|GetPlayerPawn 0)))
  (Variables|Default|Set%20Player%20Character _asbp_player_character)
  (bind _returnvalue (Game|SpawnActorfromClass "/Game/BluePrints/Building/BP_Fire.BP_Fire_C" (Math|Conversions|ToTransform(Vector) (Transformation|GetWorldLocation (Variables|Default|GetFirePont))) "Undefined" "MultiplyWithRoot" 0 false 0))
  (bind _output_get (Variables|Default|Set%20BP%20Fire _returnvalue))
  (Rendering|SetVisibility (Variables|/Game/BluePrints/Building/BP_Build.BP_Build_C|GetMesh1 _output_get) false false)
  (Rendering|SetVisibility (Variables|/Game/BluePrints/Building/BP_Build.BP_Build_C|GetMesh2 _output_get) false false))

(event Collision|EventActorBeginOverlap
  (params (OtherActor :type Actor%20Object%20Reference))
  (|CallParentFunction OtherActor) ; This node is disabled and will not be called.\nDrag off pins to build functionality.
)

(event EventTick
  (params (DeltaSeconds :type Float%20%28single-precision%29))
  (|CallParentFunction DeltaSeconds) ; This node is disabled and will not be called.\nDrag off pins to build functionality.
)

(fn ConstructionScript
  (|CallParentFunction))