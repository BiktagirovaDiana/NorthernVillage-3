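; BP_Tree is a choppable tree that the player can approach and residents can reserve.
; A Box trigger sets CanChop on BP_PlayerCharacter while the player overlaps it, and the Chop event itself is empty.
; Reserve, Release and IsFree form a single-owner lock keyed by resident row name, so only the holder can release it.
; GetChopLocation returns the world location of the ChopPoint component.
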(event OnComponentBeginOverlap(Box)
  (params (OverlappedComponent :type Primitive%20Component%20Object%20Reference) (OtherActor :type Actor%20Object%20Reference) (OtherComp :type Primitive%20Component%20Object%20Reference) (OtherBodyIndex :type Integer) (bFromSweep :type Boolean) (SweepResult :type Hit%20Result%20Structure%20%28by%20ref%29))
  (bind _asbp_player_character (Utilities|Casting|CastToBP_PlayerCharacter OtherActor))
  (Variables|/Game/BluePrints/Player/BP_PlayerCharacter.BP_PlayerCharacter_C|SetCanChop _asbp_player_character true))

(event OnComponentEndOverlap(Box)
  (params (OverlappedComponent :type Primitive%20Component%20Object%20Reference) (OtherActor :type Actor%20Object%20Reference) (OtherComp :type Primitive%20Component%20Object%20Reference) (OtherBodyIndex :type Integer))
  (bind _asbp_player_character (Utilities|Casting|CastToBP_PlayerCharacter OtherActor))
  (Variables|/Game/BluePrints/Player/BP_PlayerCharacter.BP_PlayerCharacter_C|SetCanChop _asbp_player_character false))

(event Custom|Chop)

(event EventBeginPlay)

(event Collision|EventActorBeginOverlap
  (params (OtherActor :type Actor%20Object%20Reference)))

(event EventTick
  (params (DeltaSeconds :type Float%20%28single-precision%29)))

(fn ConstructionScript)

(fn IsFree
  (return (not (Variables|Default|GetbReserved))))

(fn Reserve
  (params (ResidentRowName :type Name))
  (if (not (Variables|Default|GetbReserved))
    (Variables|Default|SetbReserved true)
    (Variables|Default|SetReservedBy ResidentRowName)
    (return true)
    (else
      (return false))))

(fn GetChopLocation
  (return (Transformation|GetWorldLocation (Variables|Default|GetChopPoint))))

(fn Release
  (params (Resident%20Row%20Name :type Name))
  (if (and (== (Variables|Default|GetbReserved) true) (== (Variables|Default|GetReservedBy) Resident%20Row%20Name))
    (Variables|Default|SetbReserved false)
    (Variables|Default|SetReservedBy "None")
    (return true)
    (else
      (return false))))