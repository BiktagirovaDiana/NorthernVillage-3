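; BP_WaterSource_IceHole is an ice hole where the player can fill water and fish, and which residents can reserve.
; It registers with BP_IceHoleManager on play and unregisters on end, while box overlap toggles the player's CanFillWater and CanFish flags.
; Reserve and IsFree track occupancy by resident row name, and GetFishingLocation exposes the fishing point.
; Release also requires IsOccupied, which the live Reserve path never sets.
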(event OnComponentBeginOverlap(Box)
  (params (OverlappedComponent :type Primitive%20Component%20Object%20Reference) (OtherActor :type Actor%20Object%20Reference) (OtherComp :type Primitive%20Component%20Object%20Reference) (OtherBodyIndex :type Integer) (bFromSweep :type Boolean) (SweepResult :type Hit%20Result%20Structure%20%28by%20ref%29))
  (bind _asbp_player_character (Utilities|Casting|CastToBP_PlayerCharacter OtherActor))
  (Variables|/Game/BluePrints/Player/BP_PlayerCharacter.BP_PlayerCharacter_C|SetCanFillWater _asbp_player_character true)
  (Variables|/Game/BluePrints/Player/BP_PlayerCharacter.BP_PlayerCharacter_C|SetCanFish _asbp_player_character true)
  (Development|PrintString (Utilities|String|ToString(Integer) (Variables|Default|GetHoleID)) true true "(R=0.000000,G=0.660000,B=1.000000,A=1.000000)" 5.0))

(event OnComponentEndOverlap(Box)
  (params (OverlappedComponent :type Primitive%20Component%20Object%20Reference) (OtherActor :type Actor%20Object%20Reference) (OtherComp :type Primitive%20Component%20Object%20Reference) (OtherBodyIndex :type Integer))
  (bind _asbp_player_character (Utilities|Casting|CastToBP_PlayerCharacter OtherActor))
  (Variables|/Game/BluePrints/Player/BP_PlayerCharacter.BP_PlayerCharacter_C|SetCanFillWater _asbp_player_character false)
  (Variables|/Game/BluePrints/Player/BP_PlayerCharacter.BP_PlayerCharacter_C|SetCanFish _asbp_player_character false))

(event EventBeginPlay
  (Variables|Default|SetbIsOccupied false)
  (Variables|Default|SetOccupiedByResident "None")
  (bind _outactors (Actor|GetAllActorsOfClass "/Game/BluePrints/Resources/BP_IceHoleManager.BP_IceHoleManager_C"))
  (if (> (Utilities|Array|Length _outactors) 0)
    (bind _asbp_ice_hole_manager (Utilities|Casting|CastToBP_IceHoleManager (Utilities|Array|Get(acopy) _outactors)))
    (Default|RegisterIceHole _asbp_ice_hole_manager self)))

(event Collision|EventActorBeginOverlap
  (params (OtherActor :type Actor%20Object%20Reference)))

(event EventTick
  (params (DeltaSeconds :type Float%20%28single-precision%29)))

(event EventEndPlay
  (params (EndPlayReason :type EEndPlayReason%20Enum :default "Destroyed"))
  (bind _outactors (Actor|GetAllActorsOfClass "/Game/BluePrints/Resources/BP_IceHoleManager.BP_IceHoleManager_C"))
  (if (> (Utilities|Array|Length _outactors) 0)
    (bind _asbp_ice_hole_manager (Utilities|Casting|CastToBP_IceHoleManager (Utilities|Array|Get(acopy) _outactors)))
    (Default|UnregisterIceHole _asbp_ice_hole_manager self)))

(fn ConstructionScript
  (if (Utilities|Enum|Equal(Enum) (Variables|Default|GetHoleName) "")
    (Variables|Default|SetHoleName (Utilities|GetDisplayName self))))

(fn IsFree
  (return (== (Variables|Default|GetOccupiedByResident) "")))

(fn Reserve
  (params (ResidentRowName :type Name))
  (Development|PrintString (Utilities|String|Append "Reserve called   " (Utilities|String|ToString(Name) (Variables|Default|GetOccupiedByResident))))
  (if (== (Variables|Default|GetOccupiedByResident) "")
    (bind _output_get (Variables|Default|SetOccupiedByResident ResidentRowName))
    (Development|PrintString (Utilities|String|ToString(Name) _output_get))
    (return true)
    (else
      (Development|PrintString "пустой")
      (return false))))

(fn Release
  (params (ResidentRowName :type Name))
  (if (and (== (Variables|Default|GetbIsOccupied) true) (== (Variables|Default|GetOccupiedByResident) ResidentRowName))
    (Variables|Default|SetbIsOccupied false)
    (Variables|Default|SetOccupiedByResident "None")))

(fn GetFishingLocation
  (return (Transformation|GetWorldLocation (Variables|Default|GetFishingPoint))))