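; Manager that tracks ice fishing holes, resident jobs and which hole each resident uses.
; Registered holes without an ID get sequential IDs and names, and job changes fire a notification, releasing the hole for non-fishermen.
; GetResidentHole returns the stored hole or picks a random free one, re-rolling per pure-node evaluation and never marking it occupied.
; AssignHoleToResident only returns existing assignments, as its assignment logic is disconnected.
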(event EventBeginPlay)

(event Collision|EventActorBeginOverlap
  (params (OtherActor :type Actor%20Object%20Reference)))

(event EventTick
  (params (DeltaSeconds :type Float%20%28single-precision%29)))

(fn ConstructionScript)

(fn RegisterIceHole
  (params (Hole :type BP%20Water%20Source%20Ice%20Hole%20Object%20Reference))
  (bind _iceholes (Variables|Default|GetIceHoles))
  (Utilities|IsValid Hole
    (:Is%20Valid
      (if (not (Utilities|Array|ContainsItem _iceholes Hole))
        (Utilities|Array|Add _iceholes Hole)
        (if (== (Variables|/Game/BluePrints/Resources/BP_WaterSource_IceHole.BP_WaterSource_IceHole_C|GetHoleID Hole) -1)
          (Variables|/Game/BluePrints/Resources/BP_WaterSource_IceHole.BP_WaterSource_IceHole_C|SetHoleID Hole (Variables|Default|GetNextHoleID))
          (Variables|/Game/BluePrints/Resources/BP_WaterSource_IceHole.BP_WaterSource_IceHole_C|SetHoleName Hole (Utilities|String|Append "Лунка" (Utilities|String|ToString(Integer) (Variables|Default|GetNextHoleID))))
          (Variables|Default|SetNextHoleID (+ (Variables|Default|GetNextHoleID) 1)))))))

(fn UnregisterIceHole
  (params (Hole :type BP%20Water%20Source%20Ice%20Hole%20Object%20Reference))
  (Utilities|Array|RemoveItem (Variables|Default|GetIceHoles) Hole))

(fn GetFreeHolesforResident
  (params (ResidentRowName :type Name))
  (Utilities|Array|Clear (LocalVariables|GetOutHolesLocal))
  (for _array_element (Variables|Default|GetIceHoles)
    (Utilities|IsValid _array_element
      (:Is%20Valid
        (if (or (not (Variables|/Game/BluePrints/Resources/BP_WaterSource_IceHole.BP_WaterSource_IceHole_C|GetbIsOccupied _array_element)) (== (Variables|/Game/BluePrints/Resources/BP_WaterSource_IceHole.BP_WaterSource_IceHole_C|GetOccupiedByResident _array_element) ResidentRowName))
          (Utilities|Array|Add (LocalVariables|GetOutHolesLocal) _array_element)))))
  (bind _output_get (Variables|Default|SetOutHoles (LocalVariables|GetOutHolesLocal)))
  (return _output_get))

(fn SetResidentJob
  (params (ResidentRowName :type Name) (NewJob :type String))
  (Utilities|Map|Add (Variables|Default|GetResidentJob) ResidentRowName NewJob)
  (Default|CallOnResidentJobChanged ResidentRowName NewJob)
  (if (Utilities|Enum|NotEqual(Enum) NewJob "Рыбак")
    (CallFunction|ClearResidentHole ResidentRowName)))

(fn ClearResidentHole
  (params (ResidentRowName :type Name))
  (bind _residenthole (Variables|Default|GetResidentHole))
  (bind _value (Utilities|Map|Find _residenthole ResidentRowName))
  (Utilities|IsValid _value
    (:Is%20Valid
      (Variables|/Game/BluePrints/Resources/BP_WaterSource_IceHole.BP_WaterSource_IceHole_C|SetbIsOccupied _value false)
      (Variables|/Game/BluePrints/Resources/BP_WaterSource_IceHole.BP_WaterSource_IceHole_C|SetOccupiedByResident _value "None")
      (Utilities|Map|Remove (Variables|Default|GetResidentHole) ResidentRowName))))

(fn GetResidentJob
  (params (ResidentRowName :type Name))
  (bind _residentjob (Variables|Default|GetResidentJob))
  (bind (_value _returnvalue) (Utilities|Map|Find _residentjob ResidentRowName))
  (if _returnvalue
    (return _value)
    (else
      (return "Безработный"))))

(fn AssignHoletoResident
  (params (ResidentRowName :type Name))
  (bind _residenthole (Variables|Default|GetResidentHole))
  (bind (_value _returnvalue) (Utilities|Map|Find _residenthole ResidentRowName))
  (if _returnvalue
    (Utilities|IsValid _value
      (:Is%20Valid
        (return _value true)))))

(fn GetResidentHole
  (params (ResidentRowName :type Name))
  (bind _residenthole (Variables|Default|GetResidentHole))
  (bind _value (Utilities|Map|Find _residenthole ResidentRowName))
  (if (Utilities|Map|Contains _residenthole ResidentRowName)
    (Utilities|IsValid _value
      (:Is%20Valid
        (return _value true))
      (:Is%20Not%20Valid
        (Utilities|Map|Remove _residenthole ResidentRowName)))
    (else
      (bind _outholes (CallFunction|GetFreeHolesforResident ResidentRowName))
      (if (> (Utilities|Array|Length _outholes) 0)
        (Utilities|IsValid (Utilities|Array|Get(acopy) _outholes (Math|Random|RandomIntegerinRange 0 (- (Utilities|Array|Length _outholes) 1)))
          (:Is%20Valid
            (Utilities|Map|Add (Variables|Default|GetResidentHole) ResidentRowName (Utilities|Array|Get(acopy) _outholes (Math|Random|RandomIntegerinRange 0 (- (Utilities|Array|Length _outholes) 1))))
            (return (Utilities|Array|Get(acopy) _outholes (Math|Random|RandomIntegerinRange 0 (- (Utilities|Array|Length _outholes) 1))) true))
          (:Is%20Not%20Valid
            (return 0 false)))
        (else
          (return 0 false))))))